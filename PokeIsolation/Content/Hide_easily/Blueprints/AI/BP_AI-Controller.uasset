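; AI controller for the hide-and-seek NPC that patrols, chases players and checks closets.
; On BeginPlay it runs BT_PatrolChaseAndSearch and copies the pawn's patrol, chase and attack settings into the Blackboard.
; Perception updates set CanSeePlayer and ChaseActor for living players within chase range.
; Helper functions map world locations to the patrol path's closets to open, close or check them for hidden players, firing dispatchers on opening and discovery.
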(event `self.ReceiveBeginPlay`
  (bind _returnvalue (`AIBlueprintHelperLibrary.GetBlackboard` null))
  (`self.RunBehaviorTree` "/Game/Hide_easily/Blueprints/AI/BT_PatrolChaseAndSearch.BT_PatrolChaseAndSearch")
  (bind _asbp_ai_character (cast `/Game/Hide_easily/Blueprints/AI/BP_AI-Character` (`self.K2_GetPawn`)))
  (set `self.NPC Pawn` _asbp_ai_character)
  (`BlackboardComponent.SetValueAsFloat` _returnvalue "Time" (`/Game/Hide_easily/Blueprints/AI/BP_AI-Character.Wait Time` (`self.NPC Pawn`)))
  (`BlackboardComponent.SetValueAsBool` _returnvalue "PathLoop" (`/Game/Hide_easily/Blueprints/AI/BP_AI-Character.Is Looping?` (`self.NPC Pawn`)))
  (`BlackboardComponent.SetValueAsInt` _returnvalue "Direction" 1)
  (`BlackboardComponent.SetValueAsFloat` _returnvalue "PatrolSpeed" (`/Game/Hide_easily/Blueprints/AI/BP_AI-Character.Patrol Speed` (`self.NPC Pawn`)))
  (`BlackboardComponent.SetValueAsFloat` _returnvalue "ChaseSpeed" (`/Game/Hide_easily/Blueprints/AI/BP_AI-Character.Chase Speed` (`self.NPC Pawn`)))
  (`BlackboardComponent.SetValueAsFloat` _returnvalue "MinDistanceToAttack" (`/Game/Hide_easily/Blueprints/AI/BP_AI-Character.Min Player Distance to Attack` (`self.NPC Pawn`)))
  (`BlackboardComponent.SetValueAsFloat` _returnvalue "MinDistanceToChase" (`/Game/Hide_easily/Blueprints/AI/BP_AI-Character.Min Player Distance to Chase` (`self.NPC Pawn`)))
  (`BlackboardComponent.SetValueAsBool` _returnvalue "KillPlayers?" (`/Game/Hide_easily/Blueprints/AI/BP_AI-Character.Kill Players?` (`self.NPC Pawn`))))

(event `self.AIPerception.OnTargetPerceptionUpdated`
  (params (Actor :type "Actor Object Reference") (Stimulus :type "AIStimulus Structure"))
  (bind (_age _expirationage _strength _stimuluslocation _receiverlocation _tag _bsuccessfullysensed) (break `AIStimulus` Stimulus))
  (bind _returnvalue (`AIBlueprintHelperLibrary.GetBlackboard` null))
  ;[1 1 1] Chase/ AI sees you
  ;;[1 1 1] is controlled by hideEasily controller?
  (bind _asbi_hide_easily_control (cast `/Game/Hide_easily/Blueprints/GameModeAndController/BI_HideEasilyControl` (`Pawn.GetController` (`Actor.Instigator` Actor))))
  (bind _dead (`/Game/Hide_easily/Blueprints/GameModeAndController/BI_HideEasilyControl.BI Get Dead` _asbi_hide_easily_control))
  (if (and (not _dead) (<= (`KismetMathLibrary.Vector_Distance` _stimuluslocation _receiverlocation) (`/Game/Hide_easily/Blueprints/AI/BP_AI-Character.Min Player Distance to Chase` (`self.NPC Pawn`))))
    (if (== (`BlackboardComponent.GetValueAsBool` _returnvalue "CanSeePlayer") true)
      (`self.OnSeeingYou`)
      (`BlackboardComponent.SetValueAsBool` _returnvalue "CanSeePlayer" _bsuccessfullysensed) ; if you hide, it stops following you
      (if (== _bsuccessfullysensed true)
        (`BlackboardComponent.SetValueAsObject` _returnvalue "ChaseActor" Actor :!label _label))
      (else
        (`BlackboardComponent.SetValueAsBool` _returnvalue "CanSeePlayer" true)
        (goto _label)))))

(fn `CanInteractWithCloset?`
  (params (Key :type "Vector Structure (by ref)"))
  (returns (ReturnValue :type Boolean))
  (bind _patrolpath (`/Game/Hide_easily/Blueprints/AI/BP_AI-Character.PatrolPath` (`self.NPC Pawn`)))
  (return (`.ReturnValue` (`BlueprintMapLibrary.Map_Find` (`/Game/Hide_easily/Blueprints/AI/BP_PatrolPathAndClosets.LocationsForClosets` _patrolpath) (`KismetMathLibrary.InverseTransformLocation` (`self.GetTransform` _patrolpath) Key)))))

(fn `CloseClosetDoors`
  (params (Key :type "Vector Structure (by ref)"))
  (bind _patrolpath (`/Game/Hide_easily/Blueprints/AI/BP_AI-Character.PatrolPath` (`self.NPC Pawn`)))
  (bind (_value _returnvalue) (`BlueprintMapLibrary.Map_Find` (`/Game/Hide_easily/Blueprints/AI/BP_PatrolPathAndClosets.LocationsForClosets` _patrolpath) (`KismetMathLibrary.InverseTransformLocation` (`self.GetTransform` _patrolpath) Key)))
  (if _returnvalue
    (`/Game/Hide_easily/Blueprints/BP_Closet_1.CloseDoors` _value)))

(fn `IsSomeoaneInCloset?`
  (params (Location :type "Vector Structure"))
  (returns (ReturnValue :type Boolean))
  (bind _patrolpath (`/Game/Hide_easily/Blueprints/AI/BP_AI-Character.PatrolPath` (`self.NPC Pawn`)))
  (bind (_value _returnvalue) (`BlueprintMapLibrary.Map_Find` (`/Game/Hide_easily/Blueprints/AI/BP_PatrolPathAndClosets.LocationsForClosets` _patrolpath) (`KismetMathLibrary.InverseTransformLocation` (`self.GetTransform` _patrolpath) Location)))
  (bind _returnvalue_2 (`KismetSystemLibrary.IsValid` (`/Game/Hide_easily/Blueprints/BP_Closet_1.UsingPlayer` _value)))
  (if _returnvalue
    (if _returnvalue_2
      ;[1 1 1] Event dispatcher
      (`self.OnPlayerIsFound`)
      (`KismetSystemLibrary.PrintString` "Hello"))
    (return _returnvalue_2)))

(fn `OpenClosetDoors`
  (params (Key :type "Vector Structure (by ref)"))
  (bind _patrolpath (`/Game/Hide_easily/Blueprints/AI/BP_AI-Character.PatrolPath` (`self.NPC Pawn`)))
  (bind (_value _returnvalue) (`BlueprintMapLibrary.Map_Find` (`/Game/Hide_easily/Blueprints/AI/BP_PatrolPathAndClosets.LocationsForClosets` _patrolpath) (`KismetMathLibrary.InverseTransformLocation` (`self.GetTransform` _patrolpath) Key)))
  (if _returnvalue
    (`/Game/Hide_easily/Blueprints/BP_Closet_1.OpenDoors` _value)
    ;[1 1 1] Open Door Event Dispatcher
    (`self.OnOpeningDoor`)))

(fn `UserConstructionScript`)