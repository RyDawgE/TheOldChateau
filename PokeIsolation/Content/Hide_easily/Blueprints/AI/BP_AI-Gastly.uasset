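; AI-controlled Gastly enemy character that plays Haunter montages in reaction to its controller and can be killed by the player.
; On BeginPlay it binds to BP_AI-Controller events for opening a door, finding the player and seeing the player, each triggering its own montage.
; When killed, it decrements the player's CurrentGhastlys count and destroys itself.
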(event `OnKilledByPlayer`
  (params (Player :type "/Game/PokeIsolationContent/Framework/Player/BP_PkO_Character Object Reference"))
  (`/Engine/EditorBlueprintResources/StandardMacros.DecrementInt` (`/Game/PokeIsolationContent/Framework/Player/BP_PkO_Character.CurrentGhastlys` Player)
    (:`  `
      (`self.K2_DestroyActor`))))

(event `self.ReceiveBeginPlay`
  (bind _asbp_ai_controller (cast `/Game/Hide_easily/Blueprints/AI/BP_AI-Controller` (`self.GetController`)))
  ;[1 1 1] Animation when he opens a door
  (add `/Game/Hide_easily/Blueprints/AI/BP_AI-Controller.OnOpeningDoor` _asbp_ai_controller (delegate `PlayOpenDoorAnimation`))
  (add `/Game/Hide_easily/Blueprints/AI/BP_AI-Controller.OnPlayerIsFound` _asbp_ai_controller (delegate `PlayHaunterAnim`))
  (add `/Game/Hide_easily/Blueprints/AI/BP_AI-Controller.OnSeeingYou` _asbp_ai_controller (delegate `PlaySeeYouAnimation`)))

(event `PlayOpenDoorAnimation`
  ;[1 1 1] Animation when he opens a door
  (`self.PlayAnimMontage` "/Game/assets/models/characters/haunter/anims/Montages/HaunterEatMontage.HaunterEatMontage"))

(event `PlaySeeYouAnimation`
  (`self.PlayAnimMontage` "/Game/assets/models/characters/haunter/anims/Montages/Haunter_Anim_pm0093_00_00_trmdl_pm0093_00_00_20300_roar01_gfbanm_Montage.Haunter_Anim_pm0093_00_00_trmdl_pm0093_00_00_20300_roar01_gfbanm_Montage" 3.0 "None"))

(event `PlayHaunterAnim`
  (`self.PlayAnimMontage` "/Game/assets/models/characters/haunter/anims/Montages/Haunter_Anim_pm0093_00_00_trmdl_pm0093_00_00_20320_refresh01_gfbanm_Montage.Haunter_Anim_pm0093_00_00_trmdl_pm0093_00_00_20320_refresh01_gfbanm_Montage" 1.0 "ScaryFace"))

(event `self.ReceiveTick`
  (params (DeltaSeconds :type "Float (single-precision)")))

(fn `UserConstructionScript`
  (`parent.UserConstructionScript`))