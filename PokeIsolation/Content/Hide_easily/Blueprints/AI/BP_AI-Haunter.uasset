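; Haunter enemy character for a hiding game, supplying the animations, scare effects and game-over trigger for the monster.
; On BeginPlay it binds montages to BP_AI-Controller events for opening doors, seeing the player and finding them.
; Other events turn it toward the player or teleport it in front of them, halting movement.
; The scary face combines a material swap, groan sound and timeline-driven morph target; Attack and Tick are empty.
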(event `self.ReceiveBeginPlay`
  (bind _asbp_ai_controller (cast `/Game/Hide_easily/Blueprints/AI/BP_AI-Controller` (`self.GetController`)))
  ;[1 1 1] Animation when he opens a door
  (add `/Game/Hide_easily/Blueprints/AI/BP_AI-Controller.OnOpeningDoor` _asbp_ai_controller (delegate `PlayOpenDoorAnimation`))
  (add `/Game/Hide_easily/Blueprints/AI/BP_AI-Controller.OnPlayerIsFound` _asbp_ai_controller (delegate `PlayHaunterAnim`))
  (add `/Game/Hide_easily/Blueprints/AI/BP_AI-Controller.OnSeeingYou` _asbp_ai_controller (delegate `PlaySeeYouAnimation`)))

(event `PlayOpenDoorAnimation`
  ;[1 1 1] Animation when he opens a door
  (`self.PlayAnimMontage` "/Game/assets/models/characters/haunter/anims/Haunter_Anim_pm0093_00_00_trmdl_pm0093_00_00_20295_eat02_end_gfbanm_Montage.Haunter_Anim_pm0093_00_00_trmdl_pm0093_00_00_20295_eat02_end_gfbanm_Montage"))

(event `PlaySeeYouAnimation`
  (`self.PlayAnimMontage` "/Game/assets/models/characters/haunter/anims/Haunter_Anim_pm0093_00_00_trmdl_pm0093_00_00_20300_roar01_gfbanm_Montage.Haunter_Anim_pm0093_00_00_trmdl_pm0093_00_00_20300_roar01_gfbanm_Montage" 3.0 "None"))

(event `PlayHaunterAnim`
  (`self.PlayAnimMontage` "/Game/assets/models/characters/haunter/anims/Haunter_Anim_pm0093_00_00_trmdl_pm0093_00_00_20320_refresh01_gfbanm_Montage.Haunter_Anim_pm0093_00_00_trmdl_pm0093_00_00_20320_refresh01_gfbanm_Montage" 1.0 "ScaryFace"))

(event `self.ReceiveTick`
  (params (DeltaSeconds :type "Float (single-precision)")))

(event `self.Attack`)

(event `self.ScareAnim`
  (`self.PlayAnimMontage` "/Game/assets/models/characters/haunter/anims/Haunter_Anim_pm0093_00_00_trmdl_pm0093_00_00_20011_defaultidle02_gfbanm_Montage.Haunter_Anim_pm0093_00_00_trmdl_pm0093_00_00_20011_defaultidle02_gfbanm_Montage" 2.0))

(event `self.ShowGameOver`
  (bind _asbp_pk_o_player_controller (cast `/Game/PokeIsolationContent/Blueprints/GameModeandController/BP_PkO_PlayerController` (`GameplayStatics.GetPlayerController` 0)))
  (`/Game/PokeIsolationContent/Blueprints/GameModeandController/BP_PkO_PlayerController.Show Game Over Screen` _asbp_pk_o_player_controller))

(event `self.Chasing`
  (`KismetSystemLibrary.Delay` 3.0)
  (`self.PlayAnimMontage` "/Game/assets/models/characters/haunter/anims/Haunter_Anim_pm0093_00_00_trmdl_pm0093_00_00_20295_eat02_end_gfbanm_Montage.Haunter_Anim_pm0093_00_00_trmdl_pm0093_00_00_20295_eat02_end_gfbanm_Montage"))

(event `self.AttackAnim`
  (`self.PlayAnimMontage` "/Game/assets/models/characters/haunter/anims/Haunter_Anim_pm0093_00_00_trmdl_pm0093_00_00_20410_attack02_gfbanm_Montage.Haunter_Anim_pm0093_00_00_trmdl_pm0093_00_00_20410_attack02_gfbanm_Montage" 2.0))

(event `self.FoundPlayer`
  (params (PlayerLocation :type "Vector Structure"))
  (`self.K2_SetActorRotation` (`KismetMathLibrary.FindLookAtRotation` (`self.K2_GetActorLocation`) PlayerLocation)))

(event `self.TeleInFrontOfPlayer`
  (params (PlayerLocation :type "Vector Structure") (PlayerForwardVector :type "Vector Structure") (Distance :type "Float (double-precision)") (bGameOver :type Boolean))
  (bind _returnvalue (`AIBlueprintHelperLibrary.GetAIController` self))
  (`self.K2_SetActorRotation` (`KismetMathLibrary.FindLookAtRotation` (`self.K2_GetActorLocation`) PlayerLocation))
  (`self.K2_SetActorLocation` (+ PlayerLocation (* PlayerForwardVector Distance)))
  (set `self.PatrolPath` null)
  (`AIController.K2_SetFocalPoint` _returnvalue PlayerLocation)
  (`Controller.StopMovement` _returnvalue))

(event `Set ScaryFace`
  (`PrimitiveComponent.SetMaterial` (`self.Mesh`) 1 "/Game/assets/models/characters/haunter/materials/SRS_Haunter_Body_Scary.SRS_Haunter_Body_Scary")
  (`GameplayStatics.PlaySoundAtLocation` "/Game/Sounds/Haunter/ES_Monster_GroanWReverb.ES_Monster_GroanWReverb" (`self.K2_GetActorLocation`) (struct) 1.0 1.0 0.0 null null null null)
  (bind (_direction _morph) (`Timeline|MorphinTime`)
    (:`Update`
      (`SkeletalMeshComponent.SetMorphTarget` (`self.Mesh`) "Scary" _morph true))))

(fn `UserConstructionScript`
  (`parent.UserConstructionScript`))