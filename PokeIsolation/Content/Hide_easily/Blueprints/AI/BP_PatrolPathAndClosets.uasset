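; Patrol path actor that inserts closet stops into its patrol points, computed in the Construction Script.
; GetClosestCloset converts each closet's CollBoxOut location to actor space and assigns it a path segment; its check only tests stored distance above zero, so later segments overwrite earlier ones.
; AddNewPoints builds FinalPoints by inserting those locations after their segment's start point, then maps each location to its closet in LocationsForClosets.
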(event `self.ReceiveBeginPlay`)

(fn `AddNewPoints`
  (for (_array_element _array_index) (`self.PathPoints`)
    (`KismetArrayLibrary.Array_Add` (`self.FinalPoints`) _array_element)
    (for (_array_element_2 _array_index_2) (`self.PathIds`)
      (if (== _array_index _array_element_2)
        (`KismetArrayLibrary.Array_Add` (`self.FinalPoints`) (`|GetArrayItem` (`self.ClosestPositionToClosets`) _array_index_2)))))
  ;[1 1 1] save location for every closet
  (for (_array_element_3 _array_index_3) (`self.Closets`)
    (`BlueprintMapLibrary.Map_Add` (`self.LocationsForClosets`) (`|GetArrayItem` (`self.ClosestPositionToClosets`) _array_index_3) _array_element_3)))

(fn `GetClosestCloset`
  (bind _pathpoints (`self.PathPoints`))
  (for (_array_element _array_index) (`self.Closets`)
    (for (_ _array_index_2) (`self.AuxPoints`)
      (if (< 0.0 (`BlueprintMapLibrary.Map_Find` (`self.ClosetsDistanceToPath`) _array_element))
        (bind _returnvalue (`KismetMathLibrary.InverseTransformLocation` (`self.GetTransform`) (`SceneComponent.K2_GetComponentLocation` (`/Game/Hide_easily/Blueprints/BP_Closet_1.CollBox_Out` _array_element))))
        (`BlueprintMapLibrary.Map_Add` (`self.ClosetsDistanceToPath`) _array_element (`KismetMathLibrary.GetPointDistanceToSegment` _returnvalue (`|GetArrayItem` _pathpoints _array_index_2) (`|GetArrayItem` _pathpoints (+ _array_index_2 1))))
        (`KismetArrayLibrary.Array_Set` (`self.PathIds`) _array_index _array_index_2)
        (`KismetArrayLibrary.Array_Set` (`self.ClosestPositionToClosets`) _array_index _returnvalue)))))

(fn `UserConstructionScript`
  (`KismetArrayLibrary.Array_Clear` (`self.FinalPoints`))
  (`KismetArrayLibrary.Array_Clear` (`self.ClosestPositionToClosets`))
  (`BlueprintMapLibrary.Map_Clear` (`self.ClosetsDistanceToPath`))
  (`BlueprintMapLibrary.Map_Clear` (`self.LocationsForClosets`))
  (for _array_element (`self.Closets`)
    (`BlueprintMapLibrary.Map_Add` (`self.ClosetsDistanceToPath`) _array_element 9.76627899281336e+18)
    (`KismetArrayLibrary.Array_Add` (`self.ClosestPositionToClosets`) (0.0 2.0 0.0))
    (`KismetArrayLibrary.Array_Add` (`self.PathIds`)))
  (bind _output_get (set `self.AuxPoints` (`self.PathPoints`)))
  (`KismetArrayLibrary.Array_Remove` _output_get (`KismetArrayLibrary.Array_LastIndex` _output_get))
  (set `self.AuxLen` (- (`KismetArrayLibrary.Array_Length` (`self.PathPoints`)) 1))
  (`self.GetClosestCloset`)
  (`self.AddNewPoints`))