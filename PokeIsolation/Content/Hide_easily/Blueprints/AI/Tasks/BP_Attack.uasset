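; Behavior tree task that performs the AI's attack on the player it is chasing.
; It sends an attack message to the controlled pawn, then reads the chased character from the blackboard and notifies its controller through the Hide Easily control interface that it is dead, passing the kill-player flag.
; It then clears the attack blackboard flag, finishes successfully and prints a debug string; a failed cast leaves the task unfinished.
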(event `self.ReceiveExecuteAI`
  (params (OwnerController :type "AIController Object Reference") (ControlledPawn :type "Pawn Object Reference"))
  (message `/Game/Hide_easily/Blueprints/AI/BPI_TriggerAnims.Attack` ControlledPawn)
  (bind _ascharacter (cast `Character` (`BTFunctionLibrary.GetBlackboardValueAsObject` (`self.BP_ChaseActor`))))
  (bind _asbi_hide_easily_control (cast `/Game/Hide_easily/Blueprints/GameModeAndController/BI_HideEasilyControl` (`Pawn.GetController` _ascharacter)))
  (`/Game/Hide_easily/Blueprints/GameModeAndController/BI_HideEasilyControl.BI You Are Dead` _asbi_hide_easily_control (`BTFunctionLibrary.GetBlackboardValueAsBool` (`self.BP_KillPlayer?`)))
  (`BTFunctionLibrary.SetBlackboardValueAsBool` (`self.BB_Attack`))
  (`self.FinishExecute` true)
  (`KismetSystemLibrary.PrintString` "u ded"))