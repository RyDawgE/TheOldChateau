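; Behavior tree task that updates an AI's chase destination and attack flag from the location of the chased character.
; If the player controller's interface reports not dead and the target is within chase range, it stores a random navigable point near the target and sets the attack flag by attack distance.
; Otherwise it clears the can-see-player flag and fails.
; Both distance thresholds come from the Blackboard.
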(event `self.ReceiveExecuteAI`
  (params (OwnerController :type "AIController Object Reference") (ControlledPawn :type "Pawn Object Reference"))
  (bind _returnvalue (`Actor.K2_GetActorLocation` (cast `Character` (`BTFunctionLibrary.GetBlackboardValueAsObject` (`self.BP_ChaseActor`)) :!pure true)))
  (bind _returnvalue_2 (`KismetMathLibrary.Vector_Distance` (`Actor.K2_GetActorLocation` ControlledPawn) _returnvalue))
  (bind _asbi_hide_easily_control (cast `/Game/Hide_easily/Blueprints/GameModeAndController/BI_HideEasilyControl` (`GameplayStatics.GetPlayerController` 0)))
  (bind _dead (`/Game/Hide_easily/Blueprints/GameModeAndController/BI_HideEasilyControl.BI Get Dead` _asbi_hide_easily_control))
  (if (and (not _dead) (<= _returnvalue_2 (`BTFunctionLibrary.GetBlackboardValueAsFloat` (`self.BP_MinDistanceToChase`))))
    (`BTFunctionLibrary.SetBlackboardValueAsVector` (`self.Vector`) (`NavigationSystemV1.K2_GetRandomLocationInNavigableRadius` _returnvalue 80.0 null null))
    (`BTFunctionLibrary.SetBlackboardValueAsBool` (`self.BP_Attack`) (<= _returnvalue_2 (`BTFunctionLibrary.GetBlackboardValueAsFloat` (`self.BP_MinDistanceToAttack`))))
    (`self.FinishExecute` true)
    (else
      (`BTFunctionLibrary.SetBlackboardValueAsBool` (`self.BP_CanSeePlayer`))
      (`self.FinishExecute` false))))