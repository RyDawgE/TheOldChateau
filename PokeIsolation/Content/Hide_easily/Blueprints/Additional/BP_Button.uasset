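; BP_Button is a clickable keypad button, apparently for a vending machine, that displays its Code on a text render.
; The construction script writes Code onto the label.
; Clicking the VendingVMCode component calls PressButton, which plays a timeline that lerps the component one unit along negative X from the location cached at BeginPlay.
; The file only animates the press and does not pass the code on.
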(event `self.ReceiveBeginPlay`
  (set `self.Relative Location` (`SceneComponent.RelativeLocation` (`self.vending_VM_Code`))))

(event `Press Button`
  (bind _relative_location (`self.Relative Location`))
  (bind (_direction _newtrack_0) (`Timeline|Button Animation Timeline` :!via `PlayFromStart`)
    (:`Update`
      (`SceneComponent.K2_SetRelativeLocation` (`self.vending_VM_Code`) (`KismetMathLibrary.VLerp` _relative_location (+ _relative_location (-1.0 0.0 0.0)) _newtrack_0) false false))))

(event `self.vending_VM_Code.OnClicked`
  (params (TouchedComponent :type "PrimitiveComponent Object Reference") (ButtonPressed :type "Key Structure"))
  (`self.Press Button`))

(fn `UserConstructionScript`
  (`TextRenderComponent.K2_SetText` (`self.TextRender`) (`KismetTextLibrary.Conv_StringToText` (`self.Code`))))