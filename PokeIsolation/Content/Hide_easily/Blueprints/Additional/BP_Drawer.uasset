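; Interactable bookshelf drawer in the hiding system that slides open and closed.
; Interact toggles OpenClose, whose OnRep plays or reverses a timeline sliding the mesh along world X from its construction-time location.
; Box overlap registers the drawer with the player's controller as a hiding place and shows or hides an icon widget through interface calls on that controller.
; Construction also sets a "Move U" material parameter on the mesh.
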(event `self.ReceiveBeginPlay`
  ;[0.06448 1 0] Begin play
  (add `self.Interact` (delegate `EventInteract`))
  (set `/Game/Hide_easily/Widgets/WBP_IconInteract.Icon` (`self.Icon`) (cast `/Game/Hide_easily/Widgets/WBP_IconInteract` (`WidgetComponent.GetUserWidgetObject` (`self.Widget`)) :!pure true)))

(event `OpenDrawer`
  (bind (_location_x _location_y _location_z) (`KismetMathLibrary.BreakVector` (`self.Location`)))
  ;[1 0.6267 0] OPEN/CLOSE DRAWER
  (bind (_direction _track_0) (`Timeline|Timeline_1` :!label _label)
    (:`Update`
      (`SceneComponent.K2_SetWorldLocation` (`self.SM_Bookshelves_Drawer`) (`KismetMathLibrary.VLerp` (`KismetMathLibrary.MakeVector` _location_x _location_y _location_z) (`KismetMathLibrary.MakeVector` (- _location_x 32.0) _location_y _location_z) _track_0) false true))))

(event `CloseDrawer`
  ;[1 0.6267 0] OPEN/CLOSE DRAWER
  (goto _label :!via `Reverse`))

(event `EventInteract`
  ;[0.06448 1 0] Begin play
  ;;[1 1 1] bind multiplayer
  (set `self.Open/Close` (not (`self.Open/Close`))))

(event `self.Box.OnComponentBeginOverlap`
  (params (OverlappedComponent :type "PrimitiveComponent Object Reference") (OtherActor :type "Actor Object Reference") (OtherComp :type "PrimitiveComponent Object Reference") (OtherBodyIndex :type Integer) (bFromSweep :type Boolean) (SweepResult :type "HitResult Structure (by ref)"))
  (`self.PlayerInteractHide` OtherActor true))

(event `self.Box.OnComponentEndOverlap`
  (params (OverlappedComponent :type "PrimitiveComponent Object Reference") (OtherActor :type "Actor Object Reference") (OtherComp :type "PrimitiveComponent Object Reference") (OtherBodyIndex :type Integer))
  (`self.PlayerRemoveInteract` OtherActor))

(event `ShowMessage`
  (params (`Hide/Unhide` :type Boolean))
  ;[0 0.1055 1] WIDGET
  ;;[1 1 1] CLIENT show/hide widget
  (set `/Game/Hide_easily/Widgets/WBP_IconInteract.Hide/Unhide` `Hide/Unhide` (cast `/Game/Hide_easily/Widgets/WBP_IconInteract` (`WidgetComponent.GetUserWidgetObject` (`self.Widget`)) :!pure true))
  (`SceneComponent.SetVisibility` (`self.Widget`) true false))

(event `Server_Show_Message`
  (params (`Player Controller` :type "/Game/Hide_easily/Blueprints/GameModeAndController/BI_HideEasilyControl Interface") (`Hide/Unhide` :type Boolean))
  ;[0 0.1055 1] WIDGET
  (`/Game/Hide_easily/Blueprints/GameModeAndController/BI_HideEasilyControl.BI Show Interact Message Drawer` `Player Controller` self `Hide/Unhide`))

(event `Server_Hide_Message`
  (params (`Player Controller` :type "/Game/Hide_easily/Blueprints/GameModeAndController/BI_HideEasilyControl Interface"))
  ;[0 0.1055 1] WIDGET
  (`/Game/Hide_easily/Blueprints/GameModeAndController/BI_HideEasilyControl.BI Hide Interact Message Drawer` `Player Controller` self))

(event `HideMessage`
  ;[0 0.1055 1] WIDGET
  ;;[1 1 1] CLIENT show/hide widget
  (`SceneComponent.SetVisibility` (`self.Widget`) false false))

(fn `CanInteract?`
  (returns (ReturnValue :type Boolean))
  (return (`SceneComponent.bVisible` (`self.Widget`))))

(fn `OnRep_Open/Close`
  (if (`self.Open/Close`)
    (`self.OpenDrawer`)
    (else
      (`self.CloseDrawer`))))

(fn `PlayerInteractHide`
  (params (Player :type "Actor Object Reference") (`Hide/Unhide` :type Boolean))
  (bind _asbi_hide_easily_control (cast `/Game/Hide_easily/Blueprints/GameModeAndController/BI_HideEasilyControl` (`self.GetInstigatorController` Player)))
  (`/Game/Hide_easily/Blueprints/GameModeAndController/BI_HideEasilyControl.BI Add Hiding Place` _asbi_hide_easily_control self)
  (`self.Server_Show_Message` _asbi_hide_easily_control `Hide/Unhide`))

(fn `PlayerRemoveInteract`
  (params (Player :type "Actor Object Reference"))
  (bind _asbi_hide_easily_control (cast `/Game/Hide_easily/Blueprints/GameModeAndController/BI_HideEasilyControl` (`self.GetInstigatorController` Player)))
  (`self.Server_Hide_Message` _asbi_hide_easily_control))

(fn `SetMaterialsUV`
  (params (`ParameterValue U` :type "Float (double-precision)"))
  (`MeshComponent.SetScalarParameterValueOnMaterials` (`self.SM_Bookshelves_Drawer`) "Move U" `ParameterValue U`))

(fn `UserConstructionScript`
  (bind _sm_bookshelves_drawer (`self.SM_Bookshelves_Drawer`))
  (`self.SetMaterialsUV` (`self.Parameter Value U`))
  (set `self.Location` (`SceneComponent.K2_GetComponentLocation` _sm_bookshelves_drawer))
  (`SceneComponent.K2_SetRelativeLocation` _sm_bookshelves_drawer (0.0 0.0 0.0) false false))