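; Bed hiding spot that lets a player slide underneath and climb back out, built for multiplayer.
; An outer collision box registers the bed with the player's controller and shows an interact icon.
; Interacting toggles between timed hide and unhide sequences, delegating movement, animation, input lock and client-side prompts to the controller through BI_HideEasilyControl.
; Hiding and Unhiding flags suppress overlap prompts mid-transition, while UsingPlayer tracks the occupant.
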(event `self.ReceiveBeginPlay`
  ;[0.06448 1 0] Begin play
  (add `self.Interact` (delegate `EventInteract`))
  ;;[1 1 1] set widget
  (set `/Game/Hide_easily/Widgets/WBP_IconInteract.Icon` (`self.Icon`) (cast `/Game/Hide_easily/Widgets/WBP_IconInteract` (`WidgetComponent.GetUserWidgetObject` (`self.Widget`)) :!pure true)))

(event `ShowMessage`
  (params (`Hide/Unhide` :type Boolean))
  ;[0 0.1055 1] WIDGET
  ;;[1 1 1] CLIENT show/hide widget
  (set `/Game/Hide_easily/Widgets/WBP_IconInteract.Hide/Unhide` `Hide/Unhide` (cast `/Game/Hide_easily/Widgets/WBP_IconInteract` (`WidgetComponent.GetUserWidgetObject` (`self.Widget`)) :!pure true))
  (`SceneComponent.SetVisibility` (`self.Widget`) true false))

(event `Server_Show_Message`
  (params (`Player Controller` :type "/Game/Hide_easily/Blueprints/GameModeAndController/BI_HideEasilyControl Interface") (`Hide/Unhide` :type Boolean))
  ;[0 0.1055 1] WIDGET
  (`/Game/Hide_easily/Blueprints/GameModeAndController/BI_HideEasilyControl.BI Show Interact Message Bed` `Player Controller` self `Hide/Unhide`))

(event `EventInteract` :!signature `self.Interact`
  (params (Pawn :type "Actor Object Reference") (Controller :type "PlayerController Object Reference"))
  ;[0.06448 1 0] Begin play
  ;;[1 1 1] bind multiplayer
  (set `self.Closed` (not (`self.Closed`)))
  (`self.HideUnhide` Pawn Controller))

(event `Server_Hide_Message`
  (params (`Player Controller` :type "/Game/Hide_easily/Blueprints/GameModeAndController/BI_HideEasilyControl Interface"))
  ;[0 0.1055 1] WIDGET
  (`/Game/Hide_easily/Blueprints/GameModeAndController/BI_HideEasilyControl.BI Hide Interact Message Bed` `Player Controller` self))

(event `HideMessage`
  ;[0 0.1055 1] WIDGET
  ;;[1 1 1] CLIENT show/hide widget
  (`SceneComponent.SetVisibility` (`self.Widget`) false false))

(event `self.CollBox_Out.OnComponentBeginOverlap`
  (params (OverlappedComponent :type "PrimitiveComponent Object Reference") (OtherActor :type "Actor Object Reference") (OtherComp :type "PrimitiveComponent Object Reference") (OtherBodyIndex :type Integer) (bFromSweep :type Boolean) (SweepResult :type "HitResult Structure (by ref)"))
  ;[0.6302 0.4924 0.4924] Correct side of bed | your actor enter collision box
  (`self.PlayerInteractHide` OtherActor))

(event `Hide`
  (params (Pawn :type "Actor Object Reference") (PlayerController :type "PlayerController Object Reference"))
  (bind _asbi_hide_easily_control (cast `/Game/Hide_easily/Blueprints/GameModeAndController/BI_HideEasilyControl` PlayerController :!pure true))
  ;[1 0.05429 0] HIDE / UNHIDE
  (`/Game/Hide_easily/Blueprints/GameModeAndController/BI_HideEasilyControl.BI Disable Player Input` _asbi_hide_easily_control)
  (`/Game/Hide_easily/Blueprints/GameModeAndController/BI_HideEasilyControl.BI Server Hide Animation` _asbi_hide_easily_control)
  (set `self.Hiding` true)
  (`self.Server_Hide_Message` _asbi_hide_easily_control)
  (`/Game/Hide_easily/Blueprints/GameModeAndController/BI_HideEasilyControl.BI Player Go Under Bed` _asbi_hide_easily_control Pawn (`SceneComponent.K2_GetComponentLocation` (`self.Location_In`)))
  (`KismetSystemLibrary.Delay` 1.3)
  (`/Game/Hide_easily/Blueprints/GameModeAndController/BI_HideEasilyControl.BI Add Hiding Place` _asbi_hide_easily_control self)
  (`KismetSystemLibrary.Delay` 1.0)
  (`self.Server_Show_Message` _asbi_hide_easily_control) ; enable unhide
  (set `self.Hiding` false))

(event `self.CollBox_Out.OnComponentEndOverlap`
  (params (OverlappedComponent :type "PrimitiveComponent Object Reference") (OtherActor :type "Actor Object Reference") (OtherComp :type "PrimitiveComponent Object Reference") (OtherBodyIndex :type Integer))
  ;[0.6302 0.4924 0.4924] Correct side of bed | your actor leave collision box
  (`self.PlayerRemoveInteract` OtherActor))

(event `Unhide`
  (params (Pawn :type "Actor Object Reference") (`Player Controller` :type "/Game/Hide_easily/Blueprints/GameModeAndController/BI_HideEasilyControl Interface"))
  ;[1 0.05429 0] HIDE / UNHIDE
  (`/Game/Hide_easily/Blueprints/GameModeAndController/BI_HideEasilyControl.BI Change Control Rotation` `Player Controller` false)
  (`/Game/Hide_easily/Blueprints/GameModeAndController/BI_HideEasilyControl.BI Disable Player Input` `Player Controller`)
  (`self.Server_Hide_Message` `Player Controller`)
  (set `self.Unhiding` true) ; to know when you start leaving the closet
  (`/Game/Hide_easily/Blueprints/GameModeAndController/BI_HideEasilyControl.BI Player Go Out Bed` `Player Controller` (`SceneComponent.K2_GetComponentLocation` (`self.Location_In`)) (`SceneComponent.K2_GetComponentLocation` (`self.Location_Out`)) Pawn)
  (`KismetSystemLibrary.Delay` 0.3)
  (`/Game/Hide_easily/Blueprints/GameModeAndController/BI_HideEasilyControl.BI Server Unhide Animation` `Player Controller`)
  (`KismetSystemLibrary.Delay` 0.2)
  (set `self.Unhiding` false) ; you left the closet
)

(fn `CanInteract?`
  (params (UsingPlayer :type "Actor Object Reference"))
  (returns (ReturnValue :type Boolean))
  (bind _usingplayer (`self.UsingPlayer`))
  (return (and (or (== UsingPlayer _usingplayer) (not (`KismetSystemLibrary.IsValid` _usingplayer))) (`SceneComponent.bVisible` (`self.Widget`)))))

(fn `HideUnhide`
  (params (Pawn :type "Actor Object Reference") (PlayerController :type "PlayerController Object Reference"))
  (if (`self.Closed`)
    (set `self.UsingPlayer` Pawn)
    (`self.Hide` Pawn PlayerController)
    (else
      (`self.Unhide` Pawn (cast `/Game/Hide_easily/Blueprints/GameModeAndController/BI_HideEasilyControl` PlayerController :!pure true))
      (set `self.UsingPlayer` null))))

(fn `PlayerInMotion?`
  (returns (ReturnValue :type Boolean))
  (return (not (or (`self.Hiding`) (`self.Unhiding`)))))

(fn `PlayerInteractHide`
  (params (Player :type "Actor Object Reference"))
  (bind _asbi_hide_easily_control (cast `/Game/Hide_easily/Blueprints/GameModeAndController/BI_HideEasilyControl` (`self.GetInstigatorController` Player)))
  (bind _returnvalue (`self.PlayerInMotion?`))
  (if _returnvalue
    (`/Game/Hide_easily/Blueprints/GameModeAndController/BI_HideEasilyControl.BI Add Hiding Place` _asbi_hide_easily_control self)
    (`self.Server_Show_Message` _asbi_hide_easily_control true)))

(fn `PlayerInteractUnhide`
  (params (Player :type "Actor Object Reference"))
  (bind _asbi_hide_easily_control (cast `/Game/Hide_easily/Blueprints/GameModeAndController/BI_HideEasilyControl` (`self.GetInstigatorController` Player)))
  (if (not (`self.Unhiding`))
    (`self.Server_Show_Message` _asbi_hide_easily_control)))

(fn `PlayerRemoveInteract`
  (params (Player :type "Actor Object Reference"))
  (bind _asbi_hide_easily_control (cast `/Game/Hide_easily/Blueprints/GameModeAndController/BI_HideEasilyControl` (`self.GetInstigatorController` Player)))
  (bind _returnvalue (`self.PlayerInMotion?`))
  (if (and (`/Game/Hide_easily/Widgets/WBP_IconInteract.Hide/Unhide` (cast `/Game/Hide_easily/Widgets/WBP_IconInteract` (`WidgetComponent.GetUserWidgetObject` (`self.Widget`)) :!pure true)) _returnvalue)
    (`self.Server_Hide_Message` _asbi_hide_easily_control)))

(fn `UserConstructionScript`)