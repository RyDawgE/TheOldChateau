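; Bookshelf hiding place that lets a player slip behind a swinging door and come back out.
; Inner and outer overlap boxes choose hide or unhide and route the icon prompt through the controller's BI_HideEasilyControl interface.
; Interact runs delay-timed sequences where the controller moves the pawn while a timeline swings the door, with Hiding/Unhiding flags blocking new prompts.
; The construction script offsets material UVs on four shelf meshes.
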(event `ShowMessage`
  (params (`Hide/Unhide` :type Boolean))
  ;[0 0.1055 1] WIDGET
  ;;[1 1 1] CLIENT show/hide widget
  (set `/Game/Hide_easily/Widgets/WBP_IconInteract.Hide/Unhide` `Hide/Unhide` (cast `/Game/Hide_easily/Widgets/WBP_IconInteract` (`WidgetComponent.GetUserWidgetObject` (`self.Widget`)) :!pure true))
  (`SceneComponent.SetVisibility` (`self.Widget`) true false))

(event `Server_Show_Message`
  (params (`Player Controller` :type "/Game/Hide_easily/Blueprints/GameModeAndController/BI_HideEasilyControl Interface") (`Hide/Unhide` :type Boolean))
  ;[0 0.1055 1] WIDGET
  (`/Game/Hide_easily/Blueprints/GameModeAndController/BI_HideEasilyControl.BI Show Interact Message Book` `Player Controller` self `Hide/Unhide`))

(event `self.ReceiveBeginPlay`
  ;[0.06448 1 0] Begin play
  (add `self.Interact` (delegate `EventInteract`))
  (set `/Game/Hide_easily/Widgets/WBP_IconInteract.Icon` (`self.Icon`) (cast `/Game/Hide_easily/Widgets/WBP_IconInteract` (`WidgetComponent.GetUserWidgetObject` (`self.Widget`)) :!pure true)))

(event `Server_Hide_Message`
  (params (`Player Controller` :type "/Game/Hide_easily/Blueprints/GameModeAndController/BI_HideEasilyControl Interface"))
  ;[0 0.1055 1] WIDGET
  (`/Game/Hide_easily/Blueprints/GameModeAndController/BI_HideEasilyControl.BI Hide Interact Message Book` `Player Controller` self))

(event `HideMessage`
  ;[0 0.1055 1] WIDGET
  ;;[1 1 1] CLIENT show/hide widget
  (`SceneComponent.SetVisibility` (`self.Widget`) false false))

(event `EventInteract` :!signature `self.Interact`
  (params (Pawn :type "Actor Object Reference") (Controller :type "PlayerController Object Reference"))
  ;[0.06448 1 0] Begin play
  ;;[1 1 1] bind multiplayer
  (`self.HideUnhide` Pawn Controller))

(event `self.BCollBox_Out.OnComponentBeginOverlap`
  (params (OverlappedComponent :type "PrimitiveComponent Object Reference") (OtherActor :type "Actor Object Reference") (OtherComp :type "PrimitiveComponent Object Reference") (OtherBodyIndex :type Integer) (bFromSweep :type Boolean) (SweepResult :type "HitResult Structure (by ref)"))
  (`self.PlayerInteractHide` OtherActor true))

(event `OpenDoors`
  ;[1 0.6267 0] OPEN/CLOSE DOORS
  (bind (_direction _track_0) (`Timeline|Timeline_0` :!label _label)
    (:`Update`
      (`SceneComponent.K2_SetRelativeRotation` (`self.SM_Bookshelves_Door`) (`KismetMathLibrary.RLerp` (struct) (struct :`Yaw` -50.0) _track_0 true) false false))))

(event `CloseDoors`
  ;[1 0.6267 0] OPEN/CLOSE DOORS
  (goto _label :!via `Reverse`))

(event `self.BCollBox_Out.OnComponentEndOverlap`
  (params (OverlappedComponent :type "PrimitiveComponent Object Reference") (OtherActor :type "Actor Object Reference") (OtherComp :type "PrimitiveComponent Object Reference") (OtherBodyIndex :type Integer))
  (`self.PlayerRemoveInteract` OtherActor))

(event `Hide`
  (params (Pawn :type "Actor Object Reference") (PlayerController :type "PlayerController Object Reference"))
  (bind _returnvalue (`SceneComponent.K2_GetComponentLocation` (`Actor.RootComponent` Pawn)))
  (bind _returnvalue_2 (`SceneComponent.K2_GetComponentLocation` (`self.Location_In`)))
  ;[1 0.05429 0] HIDE / UNHIDE
  (bind _asbi_hide_easily_control (cast `/Game/Hide_easily/Blueprints/GameModeAndController/BI_HideEasilyControl` PlayerController))
  (`/Game/Hide_easily/Blueprints/GameModeAndController/BI_HideEasilyControl.BI Update Hiding` _asbi_hide_easily_control true)
  (`/Game/Hide_easily/Blueprints/GameModeAndController/BI_HideEasilyControl.BI Disable Player Input` _asbi_hide_easily_control)
  (set `self.Hiding` true)
  (`self.Server_Hide_Message` _asbi_hide_easily_control)
  ;[1 1 1] Rotate
  (if (`self.RotateBeforeHide`)
    (`/Game/Hide_easily/Blueprints/GameModeAndController/BI_HideEasilyControl.BI Rotate To Face Doors` _asbi_hide_easily_control Pawn _returnvalue _returnvalue_2)
    (`KismetSystemLibrary.Delay` 0.2))
  (`self.OpenDoors`)
  (`KismetSystemLibrary.Delay` 0.4)
  (`/Game/Hide_easily/Blueprints/GameModeAndController/BI_HideEasilyControl.BI Player Go In` _asbi_hide_easily_control _returnvalue _returnvalue_2 Pawn "NewEnumerator1" (`self.RotateWhenHide`))
  (`KismetSystemLibrary.Delay` 0.8)
  (`self.CloseDoors`)
  (`KismetSystemLibrary.Delay` 0.8) ; wait until you get inside
  (set `self.Hiding` false)
  (`/Game/Hide_easily/Blueprints/GameModeAndController/BI_HideEasilyControl.BI Update Hiding` _asbi_hide_easily_control false))

(event `self.BCollBox_In.OnComponentBeginOverlap`
  (params (OverlappedComponent :type "PrimitiveComponent Object Reference") (OtherActor :type "Actor Object Reference") (OtherComp :type "PrimitiveComponent Object Reference") (OtherBodyIndex :type Integer) (bFromSweep :type Boolean) (SweepResult :type "HitResult Structure (by ref)"))
  (`self.PlayerInteractHide` OtherActor))

(event `self.BCollBox_In.OnComponentEndOverlap`
  (params (OverlappedComponent :type "PrimitiveComponent Object Reference") (OtherActor :type "Actor Object Reference") (OtherComp :type "PrimitiveComponent Object Reference") (OtherBodyIndex :type Integer))
  (`self.PlayerRemoveInteract` OtherActor))

(event `Unhide`
  (params (Pawn :type "Actor Object Reference") (`Player Controller` :type "/Game/Hide_easily/Blueprints/GameModeAndController/BI_HideEasilyControl Interface"))
  (bind _returnvalue (`SceneComponent.K2_GetComponentLocation` (`self.Location_In`)))
  ;[1 0.05429 0] HIDE / UNHIDE
  (`/Game/Hide_easily/Blueprints/GameModeAndController/BI_HideEasilyControl.BI Update Hiding` `Player Controller` true)
  (`self.Server_Hide_Message` `Player Controller`)
  (set `self.Unhiding` true) ; to know when you start leaving the closet
  (`/Game/Hide_easily/Blueprints/GameModeAndController/BI_HideEasilyControl.BI Pre Locate` `Player Controller` Pawn (`SceneComponent.K2_GetComponentLocation` (`Actor.RootComponent` Pawn)) _returnvalue)
  (`self.OpenDoors`)
  (`KismetSystemLibrary.Delay` 0.5)
  (`/Game/Hide_easily/Blueprints/GameModeAndController/BI_HideEasilyControl.BI Player Go Out` `Player Controller` _returnvalue (`SceneComponent.K2_GetComponentLocation` (`self.Location_Out`)) Pawn "NewEnumerator0")
  (`KismetSystemLibrary.Delay` 0.5)
  (`self.CloseDoors`)
  (`KismetSystemLibrary.Delay` 0.8)
  (set `self.Unhiding` false) ; you left the closet
  (`/Game/Hide_easily/Blueprints/GameModeAndController/BI_HideEasilyControl.BI Update Hiding` `Player Controller` false))

(fn `CanInteract?`
  (returns (ReturnValue :type Boolean))
  (return (`SceneComponent.bVisible` (`self.Widget`))))

(fn `HideUnhide`
  (params (Pawn :type "Actor Object Reference") (PlayerController :type "PlayerController Object Reference"))
  (if (`self.Closed`)
    (`self.Hide` Pawn PlayerController)
    (else
      (`self.Unhide` Pawn (cast `/Game/Hide_easily/Blueprints/GameModeAndController/BI_HideEasilyControl` PlayerController :!pure true)))))

(fn `PlayerInMotion?`
  (returns (ReturnValue :type Boolean))
  (return (not (or (`self.Hiding`) (`self.Unhiding`)))))

(fn `PlayerInteractHide`
  (params (Player :type "Actor Object Reference") (`Hide/Unhide` :type Boolean))
  (bind _asbi_hide_easily_control (cast `/Game/Hide_easily/Blueprints/GameModeAndController/BI_HideEasilyControl` (`self.GetInstigatorController` Player)))
  (bind _returnvalue (`self.PlayerInMotion?`))
  (if _returnvalue
    (`/Game/Hide_easily/Blueprints/GameModeAndController/BI_HideEasilyControl.BI Add Hiding Place` _asbi_hide_easily_control self)
    (set `self.Closed` `Hide/Unhide`)
    (`self.Server_Show_Message` _asbi_hide_easily_control `Hide/Unhide`)))

(fn `PlayerInteractUnhide`
  (params (Player :type "Actor Object Reference"))
  (bind _asbi_hide_easily_control (cast `/Game/Hide_easily/Blueprints/GameModeAndController/BI_HideEasilyControl` (`self.GetInstigatorController` Player)))
  (if (not (`self.Unhiding`))
    (`self.Server_Show_Message` _asbi_hide_easily_control)))

(fn `PlayerRemoveInteract`
  (params (Player :type "Actor Object Reference"))
  (bind _asbi_hide_easily_control (cast `/Game/Hide_easily/Blueprints/GameModeAndController/BI_HideEasilyControl` (`self.GetInstigatorController` Player)))
  (`self.Server_Hide_Message` _asbi_hide_easily_control))

(fn `SetMaterialsUV`
  (bind _sm_bookshelves_hl2 (`self.SM_Bookshelves_HL2`))
  (bind _sm_bookshelves_hr1 (`self.SM_Bookshelves_HR1`))
  (bind _sm_bookshelves_hr2 (`self.SM_Bookshelves_HR2`))
  (bind _sm_bookshelves_hl1 (`self.SM_Bookshelves_HL1`))
  (`|ExecutionSequence`
    (:`then_0`
      (`MeshComponent.SetScalarParameterValueOnMaterials` _sm_bookshelves_hl2 "Move U" 0.25)
      (`MeshComponent.SetScalarParameterValueOnMaterials` _sm_bookshelves_hr1 "Move U" 0.25)
      (`MeshComponent.SetScalarParameterValueOnMaterials` _sm_bookshelves_hr2 "Move U" 0.36)
      (`MeshComponent.SetScalarParameterValueOnMaterials` _sm_bookshelves_hl1 "Move U" 0.36))
    (:`then_1`
      (`MeshComponent.SetScalarParameterValueOnMaterials` _sm_bookshelves_hl2 "Move V" 0.5)
      (`MeshComponent.SetScalarParameterValueOnMaterials` _sm_bookshelves_hr1 "Move V" 0.54)
      (`MeshComponent.SetScalarParameterValueOnMaterials` _sm_bookshelves_hr2 "Move V" 0.5)
      (`MeshComponent.SetScalarParameterValueOnMaterials` _sm_bookshelves_hl1 "Move V" 0.54))))

(fn `UserConstructionScript`
  (`self.SetMaterialsUV`))