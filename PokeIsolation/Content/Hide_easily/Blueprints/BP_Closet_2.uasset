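; BP_Closet_2 is a closet hiding spot with a sliding left door, built on a parent Blueprint whose right doorknob it removes.
; A timeline slides the door, with length and curve set by the Normal or Fast hide speed.
; Hide disables input through the BI_HideEasilyControl controller interface, optionally rotates the pawn, then uses speed-based delays to open, move the player inside, close and enable unhiding.
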(event `self.OpenDoors`
  ;[1 1 1] OPEN/CLOSE DOR
  (bind (_direction _track_0) (`Timeline|New Open/close Door` :!label _label)
    (:`Update`
      (`SceneComponent.K2_SetRelativeLocation` (`self.LeftDoorRoot`) (`KismetMathLibrary.VLerp` (12.0 73.0 0.0) (12.0 -0.0 0.0) _track_0) false true))))

(event `self.CloseDoors`
  ;[1 1 1] OPEN/CLOSE DOR
  (goto _label :!via `Reverse`))

(event `self.Hide`
  (params (Pawn :type "Actor Object Reference") (PlayerController :type "PlayerController Object Reference"))
  (bind _asbi_hide_easily_control (cast `/Game/Hide_easily/Blueprints/GameModeAndController/BI_HideEasilyControl` PlayerController :!pure true))
  (bind _hidespeed (`self.HideSpeed`))
  (bind _value (`BlueprintMapLibrary.Map_Find` (`self.Delays`) _hidespeed))
  (bind _returnvalue (`SceneComponent.K2_GetComponentLocation` (`Actor.RootComponent` Pawn)))
  (bind _returnvalue_2 (`SceneComponent.K2_GetComponentLocation` (`self.Location_In`)))
  (bind _returnvalue_3 (+ _value 0.2))
  ;[1 0.1108 0] change original delay
  (`/Game/Hide_easily/Blueprints/GameModeAndController/BI_HideEasilyControl.BI Update Hiding` _asbi_hide_easily_control true)
  (`/Game/Hide_easily/Blueprints/GameModeAndController/BI_HideEasilyControl.BI Disable Player Input` _asbi_hide_easily_control)
  (set `self.Hiding` true)
  (`self.Server_Hide_Message` _asbi_hide_easily_control)
  ;[1 1 1] Rotate
  (if (`self.RotateBeforeHide`)
    (`/Game/Hide_easily/Blueprints/GameModeAndController/BI_HideEasilyControl.BI Rotate To Face Doors` _asbi_hide_easily_control Pawn _returnvalue _returnvalue_2)
    (`KismetSystemLibrary.Delay` 0.2))
  (`self.OpenDoors`)
  (`KismetSystemLibrary.Delay` _value)
  (`/Game/Hide_easily/Blueprints/GameModeAndController/BI_HideEasilyControl.BI Player Go In` _asbi_hide_easily_control _returnvalue _returnvalue_2 Pawn _hidespeed (`self.RotateWhenHide`))
  (`KismetSystemLibrary.Delay` _returnvalue_3)
  (`self.CloseDoors`)
  (`KismetSystemLibrary.Delay` (+ _returnvalue_3 0.31)) ; wait until you get inside
  (`self.Server_Show_Message` _asbi_hide_easily_control) ; enable unhide
  (set `self.Hiding` false)
  (`/Game/Hide_easily/Blueprints/GameModeAndController/BI_HideEasilyControl.BI Update Hiding` _asbi_hide_easily_control false))

(fn `SetHideSpeed`
  (bind _new_open_close_door (`self.New Open/close Door`))
  (bind _hidespeed (`self.HideSpeed`))
  (`TimelineComponent.SetTimelineLength` _new_open_close_door (select `/Game/Hide_easily/Blueprints/GameModeAndController/E_HideSpeed` _hidespeed :`NewEnumerator0` 0.7 :`NewEnumerator1` 0.5))
  (`TimelineComponent.SetFloatCurve` _new_open_close_door (select `/Game/Hide_easily/Blueprints/GameModeAndController/E_HideSpeed` _hidespeed :`NewEnumerator0` "/Game/Hide_easily/Curves/C_Point7.C_Point7" :`NewEnumerator1` "/Game/Hide_easily/Curves/C_Point5.C_Point5" :!type "CurveFloat Object Reference") "Track_0"))

(fn `UserConstructionScript`
  (`parent.UserConstructionScript`)
  (`ActorComponent.K2_DestroyComponent` (`self.RightDoorknob`)))