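; BP_Closet_3 is a single-door closet variant that inherits from a parent Blueprint, apparently for a hiding mechanic.
; Its construction script runs the parent's, then destroys the left door root, mesh and knob.
; OpenDoors and CloseDoors play and reverse a timeline that swings the remaining right door by rotator interpolation.
; SetHideSpeed selects that timeline's length and float curve for Normal or Fast hiding.
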(event `self.OpenDoors`
  ;[1 1 1] OPEN/CLOSE DORS  overwrite
  (bind (_direction _track_0) (`Timeline|New Open/Close Doors` :!label _label)
    (:`Update`
      (`SceneComponent.K2_SetRelativeRotation` (`self.RightDoorRoot`) (`KismetMathLibrary.RLerp` (struct :`Pitch` 90.0 :`Yaw` 180.0 :`Roll` 180.0) (struct :`Pitch` 90.0 :`Yaw` 75.0 :`Roll` 180.0) _track_0 true) false false))))

(event `self.CloseDoors`
  ;[1 1 1] OPEN/CLOSE DORS  overwrite
  (goto _label :!via `Reverse`))

(fn `SetHideSpeed`
  (bind _new_open_close_doors (`self.New Open/Close Doors`))
  (bind _hidespeed (`self.HideSpeed`))
  (`TimelineComponent.SetTimelineLength` _new_open_close_doors (select `/Game/Hide_easily/Blueprints/GameModeAndController/E_HideSpeed` _hidespeed :`NewEnumerator0` 0.7 :`NewEnumerator1` 0.5))
  (`TimelineComponent.SetFloatCurve` _new_open_close_doors (select `/Game/Hide_easily/Blueprints/GameModeAndController/E_HideSpeed` _hidespeed :`NewEnumerator0` "/Game/Hide_easily/Curves/C_Point7.C_Point7" :`NewEnumerator1` "/Game/Hide_easily/Curves/C_Point5.C_Point5" :!type "CurveFloat Object Reference") "Track_0"))

(fn `UserConstructionScript`
  (`parent.UserConstructionScript`)
  (`ActorComponent.K2_DestroyComponent` (`self.LeftDoorRoot`))
  (`ActorComponent.K2_DestroyComponent` (`self.LeftDoorMesh`))
  (`ActorComponent.K2_DestroyComponent` (`self.LeftDoorknob`)))