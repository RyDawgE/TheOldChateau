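; Player controller for a hide-from-monster game, handling hiding in closets, beds, bookshelves and drawers, plus death and win screens.
; Interact input type-checks the target and forwards to its server interact call, while interface events relay prompts, input locking and animations.
; Timelines lerp pawn location and rotation for entering and exiting, with selectable closet speeds.
; Game over turns the view to the teleported monster, flickers the flashlight and triggers a scare.
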(event `ServerHideAnimation`
  ;[1 0.1704 0.03063] Hide under bed animations
  ;;[0.02083 0 0] Pawn Interface Calls
  (`/Game/Hide_easily/Blueprints/HideUnderBed/BI_HideUnderBed.RunHide` (cast `/Game/Hide_easily/Blueprints/HideUnderBed/BI_HideUnderBed` (`GameplayStatics.GetPlayerCharacter` 0) :!pure true)))

(event `ClientSetLoc`
  (params (Target :type "SceneComponent Object Reference") (NewLocation :type "Vector Structure"))
  ;[1 0.1704 0.03063] Hide under bed animations
  (`SceneComponent.K2_SetWorldLocation` Target NewLocation false true))

(event `ServerSetAnimationMode`
  ;[1 0.1704 0.03063] Hide under bed animations
  ;;[0.02083 0 0] Pawn Interface Calls
  (`/Game/Hide_easily/Blueprints/HideUnderBed/BI_HideUnderBed.SetAnimationMode` (cast `/Game/Hide_easily/Blueprints/HideUnderBed/BI_HideUnderBed` (`GameplayStatics.GetPlayerCharacter` 0) :!pure true)))

(event `ClientSetRot`
  (params (Target :type "SceneComponent Object Reference") (NewRotation :type "Rotator Structure"))
  ;[1 0.1704 0.03063] Hide under bed animations
  (`SceneComponent.K2_SetWorldRotation` Target NewRotation false true))

(event `ServerUnhideAnimation`
  ;[1 0.1704 0.03063] Hide under bed animations
  ;;[0.02083 0 0] Pawn Interface Calls
  (`/Game/Hide_easily/Blueprints/HideUnderBed/BI_HideUnderBed.RunUnhide` (cast `/Game/Hide_easily/Blueprints/HideUnderBed/BI_HideUnderBed` (`GameplayStatics.GetPlayerCharacter` 0) :!pure true)))

(event `ChangeControlRotation`
  (params (UsePawnControlRotation :type Boolean))
  ;[1 0.1704 0.03063] Hide under bed animations
  ;;[0.02083 0 0] Pawn Interface Calls
  (`/Game/Hide_easily/Blueprints/HideUnderBed/BI_HideUnderBed.ChangeControl` (cast `/Game/Hide_easily/Blueprints/HideUnderBed/BI_HideUnderBed` (`GameplayStatics.GetPlayerCharacter` 0) :!pure true) UsePawnControlRotation))

(event `ShowInteractMessage`
  (params (Closet :type "/Game/Hide_easily/Blueprints/BP_Closet_1 Object Reference") (`Hide/Unhide` :type Boolean))
  ;[1 1 1] INTERACT MESSAGE
  (`/Engine/EditorBlueprintResources/StandardMacros.IsValid` Closet
    (:`Is Valid`
      (`/Game/Hide_easily/Blueprints/BP_Closet_1.ShowMessage` Closet `Hide/Unhide`))))

(event `ShowInteractMessageBed`
  (params (Bed :type "/Game/Hide_easily/Blueprints/BP_Bed Object Reference") (`Hide/Unhide` :type Boolean))
  ;[1 1 1] INTERACT MESSAGE
  (`/Engine/EditorBlueprintResources/StandardMacros.IsValid` Bed
    (:`Is Valid`
      (`/Game/Hide_easily/Blueprints/BP_Bed.ShowMessage` Bed `Hide/Unhide`))))

(event `ShowInteractMessageBook`
  (params (Bookshelves :type "/Game/Hide_easily/Blueprints/BP_Bookshelves Object Reference") (`Hide/Unhide` :type Boolean))
  ;[1 1 1] INTERACT MESSAGE
  (`/Engine/EditorBlueprintResources/StandardMacros.IsValid` Bookshelves
    (:`Is Valid`
      (`/Game/Hide_easily/Blueprints/BP_Bookshelves.ShowMessage` Bookshelves `Hide/Unhide`))))

(event `ShowInteractMessageDrawer`
  (params (Drawer :type "/Game/Hide_easily/Blueprints/Additional/BP_Drawer Object Reference") (`Hide/Unhide` :type Boolean))
  ;[1 1 1] INTERACT MESSAGE
  (`/Engine/EditorBlueprintResources/StandardMacros.IsValid` Drawer
    (:`Is Valid`
      (`/Game/Hide_easily/Blueprints/Additional/BP_Drawer.ShowMessage` Drawer `Hide/Unhide`))))

(event `HideInteractMessage`
  (params (Closet :type "/Game/Hide_easily/Blueprints/BP_Closet_1 Object Reference"))
  ;[1 1 1] INTERACT MESSAGE
  (`/Engine/EditorBlueprintResources/StandardMacros.IsValid` Closet
    (:`Is Valid`
      (`/Game/Hide_easily/Blueprints/BP_Closet_1.HideMessage` Closet))))

(event `HideInteractMessageBed`
  (params (Bed :type "/Game/Hide_easily/Blueprints/BP_Bed Object Reference"))
  ;[1 1 1] INTERACT MESSAGE
  (`/Engine/EditorBlueprintResources/StandardMacros.IsValid` Bed
    (:`Is Valid`
      (`/Game/Hide_easily/Blueprints/BP_Bed.HideMessage` Bed))))

(event `HideInteractMessageBook`
  (params (Bookshelves :type "/Game/Hide_easily/Blueprints/BP_Bookshelves Object Reference"))
  ;[1 1 1] INTERACT MESSAGE
  (`/Engine/EditorBlueprintResources/StandardMacros.IsValid` Bookshelves
    (:`Is Valid`
      (`/Game/Hide_easily/Blueprints/BP_Bookshelves.HideMessage` Bookshelves))))

(event `HideInteractMessageDrawer`
  (params (Drawer :type "/Game/Hide_easily/Blueprints/Additional/BP_Drawer Object Reference"))
  ;[1 1 1] INTERACT MESSAGE
  (`/Engine/EditorBlueprintResources/StandardMacros.IsValid` Drawer
    (:`Is Valid`
      (`/Game/Hide_easily/Blueprints/Additional/BP_Drawer.HideMessage` Drawer))))

(event `EnablePlayerInput`
  ;[0 1 0.7036] input
  (`self.EnableInput` (`GameplayStatics.GetPlayerPawn` 0) (`GameplayStatics.GetPlayerController` 0)))

(event `ToggleHideEvent`
  (params (InputObject :type "Object Object Reference"))
  (bind _returnvalue (`GameplayStatics.GetPlayerPawn` 0))
  (bind _returnvalue_2 (`GameplayStatics.GetPlayerPawn` 0))
  ;[0.3577 1 0.9102] Key
  (`/Engine/EditorBlueprintResources/StandardMacros.IsValid` InputObject
    (:`Is Valid`
      (bind _asbp_closet_1 (cast `/Game/Hide_easily/Blueprints/BP_Closet_1` InputObject)
        (:`then`
          ;;[1 1 1] closet
          (bind _returnvalue_3 (`/Game/Hide_easily/Blueprints/BP_Closet_1.CanInteract?` _asbp_closet_1 _returnvalue_2))
          (if _returnvalue_3
            (`self.InteractSERVERCloset` _asbp_closet_1 _returnvalue_2 (`GameplayStatics.GetPlayerController` 0))))
        (:`CastFailed`
          ;;[1 1 1] bed
          (bind _asbp_bed (cast `/Game/Hide_easily/Blueprints/BP_Bed` InputObject)
            (:`then`
              (bind _returnvalue_4 (`/Game/Hide_easily/Blueprints/BP_Bed.CanInteract?` _asbp_bed _returnvalue))
              (if _returnvalue_4
                (`self.InteractSERVERBed` _asbp_bed _returnvalue (`GameplayStatics.GetPlayerController` 0))))
            (:`CastFailed`
              ;;[1 1 1] book
              (bind _asbp_bookshelves (cast `/Game/Hide_easily/Blueprints/BP_Bookshelves` InputObject)
                (:`then`
                  (bind _returnvalue_5 (`/Game/Hide_easily/Blueprints/BP_Bookshelves.CanInteract?` _asbp_bookshelves))
                  (if _returnvalue_5
                    (`self.InteractSERVERBook` _asbp_bookshelves (`GameplayStatics.GetPlayerPawn` 0) (`GameplayStatics.GetPlayerController` 0))))
                (:`CastFailed`
                  ;;[1 1 1] drawer
                  (bind _asbp_drawer (cast `/Game/Hide_easily/Blueprints/Additional/BP_Drawer` InputObject))
                  (bind _returnvalue_6 (`/Game/Hide_easily/Blueprints/Additional/BP_Drawer.CanInteract?` _asbp_drawer))
                  (if _returnvalue_6
                    (`self.InteractSERVERDrawer` _asbp_drawer)))))))))))

(event `PlayerGo_Under_Bed`
  (params (Pawn :type "Actor Object Reference") (B :type "Vector Structure"))
  (bind _rootcomponent (`Actor.RootComponent` Pawn))
  (bind (_pawnlocation_x _pawnlocation_y _pawnlocation_z) (`KismetMathLibrary.BreakVector` (`self.PawnLocation`)))
  (bind _returnvalue (`SceneComponent.K2_GetComponentRotation` _rootcomponent))
  ;[1 0.1704 0.03063] Hide under bed animations
  ;;[0.03712 0.08854 0] Hide under bed
  (set `self.PlayerPawn` Pawn)
  (set `self.BedLocation` B)
  (set `Pawn.bUseControllerRotationYaw` false (cast `Pawn` Pawn :!pure true))
  (bind _output_get (set `self.PawnLocation` (`SceneComponent.K2_GetComponentLocation` _rootcomponent)))
  (bind _returnvalue_2 (`self.Get Look At Rotation` _output_get (`self.BedLocation`) _returnvalue))
  (set `self.UnderBedRotation` _returnvalue_2)
  (set `self.Relative Rotation` _returnvalue) ; save start rotation
  ;;[1 1 1] Move character down before hide
  (set `self.PrelocateBeforeHide` (`KismetMathLibrary.MakeVector` _pawnlocation_x _pawnlocation_y (- _pawnlocation_z 40.0)))
  (bind (_direction _track_0) (`Timeline|Timeline_5` :!via `PlayFromStart`)
    (:`Update`
      (`self.ClientSetLoc` _rootcomponent (`KismetMathLibrary.VLerp` (`self.PawnLocation`) (`self.PrelocateBeforeHide`) _track_0)))
    (:`Finished`
      (bind (_direction_2 _track_0_2) (`Timeline|Timeline_1` :!via `PlayFromStart`)
        (:`Update`
          (`SceneComponent.K2_SetWorldRotation` _rootcomponent (`KismetMathLibrary.RLerp` (`self.Relative Rotation`) (`self.UnderBedRotation`) _track_0_2 true) false true)
          (`self.ClientSetLoc` _rootcomponent (`KismetMathLibrary.VLerp` (`self.PrelocateBeforeHide`) (`self.BedLocation`) _track_0_2)))))))

(event `InteractSERVERCloset`
  (params (Closet :type "/Game/Hide_easily/Blueprints/BP_Closet_1 Object Reference") (Pawn :type "Actor Object Reference") (Controller :type "PlayerController Object Reference"))
  ;[0.3577 1 0.9102] Key
  (`/Game/Hide_easily/Blueprints/BP_Closet_1.Interact` Closet Pawn Controller))

(event `DisablePlayerInput`
  ;[0 1 0.7036] input
  (`self.DisableInput` (`GameplayStatics.GetPlayerPawn` 0) (`GameplayStatics.GetPlayerController` 0)))

(event `InteractSERVERBed`
  (params (Bed :type "/Game/Hide_easily/Blueprints/BP_Bed Object Reference") (Pawn :type "Actor Object Reference") (Controller :type "PlayerController Object Reference"))
  ;[0.3577 1 0.9102] Key
  (`/Game/Hide_easily/Blueprints/BP_Bed.Interact` Bed Pawn Controller))

(event `EnableRotationAndInput`
  ;[1 0.1704 0.03063] Hide under bed animations
  (set `Pawn.bUseControllerRotationYaw` true (cast `Pawn` (`self.PlayerPawn`) :!pure true))
  (`self.EnablePlayerInput`))

(event `InteractSERVERBook`
  (params (Bookshelves :type "/Game/Hide_easily/Blueprints/BP_Bookshelves Object Reference") (Pawn :type "Actor Object Reference") (Controller :type "PlayerController Object Reference"))
  ;[0.3577 1 0.9102] Key
  (`/Game/Hide_easily/Blueprints/BP_Bookshelves.Interact` Bookshelves Pawn Controller))

(event `AdjustsAfterHide`
  (bind (_bedlocation_x _bedlocation_y) (`KismetMathLibrary.BreakVector` (`self.BedLocation`)))
  (bind _playerpawn (`self.PlayerPawn`))
  (bind _aspawn (cast `Pawn` _playerpawn :!pure true))
  (bind _rootcomponent (`Actor.RootComponent` _playerpawn))
  (bind (_returnvalue_x _returnvalue_y _returnvalue_z) (`KismetMathLibrary.BreakVector` (`SceneComponent.K2_GetComponentLocation` _rootcomponent)))
  ;[1 0.1704 0.03063] Hide under bed animations
  (`self.EnablePlayerInput`)
  (`SceneComponent.K2_SetWorldLocation` _rootcomponent (`KismetMathLibrary.MakeVector` _bedlocation_x _bedlocation_y (- _returnvalue_z 105.0)) false true)
  (set `Pawn.bUseControllerRotationYaw` true _aspawn)
  (`self.SetControlRotation` (`self.GetInstigatorController` _aspawn) (`self.UnderBedRotation`)))

(event `InteractSERVERDrawer`
  (params (Drawer :type "/Game/Hide_easily/Blueprints/Additional/BP_Drawer Object Reference"))
  ;[0.3577 1 0.9102] Key
  (`/Game/Hide_easily/Blueprints/Additional/BP_Drawer.Interact` Drawer))

(event `AdjustsAfterUnhide`
  (bind _playerpawn (`self.PlayerPawn`))
  ;[1 0.1704 0.03063] Hide under bed animations
  (`SceneComponent.K2_SetWorldLocation` (`Actor.RootComponent` _playerpawn) (`self.OutsideLocation`) false true)
  (`self.SetControlRotation` (`self.GetInstigatorController` _playerpawn) (`self.EndRotation`)))

(event `PlayerGo_Out`
  (params (A :type "Vector Structure") (B :type "Vector Structure") (Pawn :type "Actor Object Reference") (Speed :type "/Game/Hide_easily/Blueprints/GameModeAndController/E_HideSpeed Enum" :default "NewEnumerator0"))
  ;[0.9286 0.5318 1] come out of the closet // you call it inside Unhide event RED
  (`self.SetUnhidingSpeed` Speed)
  (bind (_direction _track_0) (`Timeline|GoOutClosetTimer` :!via `PlayFromStart`)
    (:`Update`
      (`SceneComponent.K2_SetWorldLocation` (`Actor.RootComponent` Pawn) (`KismetMathLibrary.VLerp` A B _track_0) false true))))

(event `PreLocate`
  (params (Pawn :type "Actor Object Reference") (A :type "Vector Structure") (B :type "Vector Structure"))
  ;[0.9286 0.5318 1] from player location to start in/out location  [for BP_Bookshelves]
  (bind (_direction _track_0) (`Timeline|Timeline_0` :!via `PlayFromStart`)
    (:`Update`
      (`SceneComponent.K2_SetWorldLocation` (`Actor.RootComponent` Pawn) (`KismetMathLibrary.VLerp` A B _track_0) false true))))

(event `PlayerGo_Out_Bed`
  (params (A :type "Vector Structure") (B :type "Vector Structure") (Pawn :type "Actor Object Reference"))
  (bind _aspawn (cast `Pawn` Pawn :!pure true))
  (bind _rootcomponent (`Actor.RootComponent` Pawn))
  ;[1 0.1704 0.03063] Hide under bed animations
  ;;[0.03712 0.08854 0] Unhide bed
  (`SceneComponent.K2_SetWorldLocation` (`Actor.RootComponent` _aspawn) (+ A (0.0 0.0 17.0)) false true)
  (set `self.OutsideLocation` B)
  (set `Pawn.bUseControllerRotationYaw` false _aspawn)
  (bind _output_get (set `self.Relative Rotation` (`SceneComponent.K2_GetComponentRotation` _rootcomponent))) ; save start rotation
  (bind _returnvalue (`self.Get Look At Rotation` A B _output_get))
  (bind _output_get_2 (set `self.EndRotation` _returnvalue))
  (bind (_direction _newtrack_0) (`Timeline|Timeline_3` :!via `PlayFromStart`)
    (:`Update`
      (bind _returnvalue_2 (`KismetMathLibrary.RLerp` (`self.Relative Rotation`) _output_get_2 _newtrack_0 true))
      (`SceneComponent.K2_SetWorldRotation` _rootcomponent _returnvalue_2 true true)
      (`self.ClientSetRot` _rootcomponent _returnvalue_2))
    (:`Finished`
      ;;;[1 1 1] Move character forward before unhide
      (bind _returnvalue_3 (`self.GetMidLocation` A B 0.4))
      (set `self.PrelocateBeforeHide` _returnvalue_3)
      (bind (_direction_2 _track_0) (`Timeline|Timeline_6` :!via `PlayFromStart`)
        (:`Update`
          (`self.ClientSetLoc` _rootcomponent (`KismetMathLibrary.VLerp` A (`self.PrelocateBeforeHide`) _track_0)))
        (:`Finished`
          (bind (_direction_3 _newtrack_0_2) (`Timeline|Timeline_2` :!via `PlayFromStart`)
            (:`Update`
              (`self.ClientSetLoc` _rootcomponent (`KismetMathLibrary.VLerp` (`self.PrelocateBeforeHide`) B _newtrack_0_2)))))))))

(event `PlayerRotateToFaceDoors`
  (params (Pawn :type "Actor Object Reference") (Player :type "Vector Structure") (Target :type "Vector Structure"))
  (bind _returnvalue (`SceneComponent.K2_GetComponentRotation` (`Actor.RootComponent` Pawn)))
  ;[0.295 0.169 0.3177] Turn around so you can see the doors
  (`self.ChangeControlRotation` false)
  (bind _returnvalue_2 (`self.Get Look At Rotation` Player Target _returnvalue))
  (set `self.EndRotation` _returnvalue_2)
  (bind _output_get (set `self.Relative Rotation` _returnvalue))
  (bind (_direction _newtrack_0) (`Timeline|Timeline_4` :!via `PlayFromStart`)
    (:`Update`
      (`self.SetControlRotation` (`self.GetInstigatorController` (cast `Pawn` Pawn :!pure true)) (`KismetMathLibrary.RLerp` _output_get (`self.EndRotation`) _newtrack_0 true)))
    (:`Finished`
      (`self.ChangeControlRotation` true))))

(event `Print Message`
  (params (InString :type String))
  ;[0 1 0.25] AI Widget Interactions (Death and stuff)
  (`KismetSystemLibrary.PrintString` InString))

(event `YouAreDead`
  (params (`Kill player?` :type Boolean))
  ;[0 1 0.25] AI Widget Interactions (Death and stuff)
  (`self.ShowScreenMessage` `Kill player?`)
  (`self.PlayerDead` `Kill player?`))

(event `PlayerDead`
  (params (`Dead?` :type Boolean))
  ;[0 1 0.25] AI Widget Interactions (Death and stuff)
  (set `self.Dead?` `Dead?`))

(event `PlayerGo_In`
  (params (A :type "Vector Structure") (B :type "Vector Structure") (Pawn :type "Actor Object Reference") (Speed :type "/Game/Hide_easily/Blueprints/GameModeAndController/E_HideSpeed Enum" :default "NewEnumerator0") (`Rotate?` :type Boolean))
  ;[1 1 1] Go In/Rotate Go In
  ;;[0.9286 0.5318 1] enter the closet  // you call it inside Hide event RED
  (if `Rotate?`
    (`self.PlayerGo_InRotate` A B Pawn Speed)
    (else
      (`self.SetHidingSpeed` Speed)
      (message `/Game/Hide_easily/Blueprints/HideUnderBed/BI_HideUnderBed.StopFootsteps` Pawn)
      (`self.EnablePlayerInput`)
      (bind (_direction _track_0) (`Timeline|GoInClosetTimer` :!via `PlayFromStart`)
        (:`Update`
          (`SceneComponent.K2_SetWorldLocation` (`Actor.RootComponent` Pawn) (`KismetMathLibrary.VLerp` A B _track_0) false true))))))

(event `/Game/Hide_easily/Blueprints/GameModeAndController/BI_HideEasilyControl.BI Player Go In`
  (params (A :type "Vector Structure") (B :type "Vector Structure") (Pawn :type "Actor Object Reference") (Speed :type "/Game/Hide_easily/Blueprints/GameModeAndController/E_HideSpeed Enum" :default "NewEnumerator0") (`Rotate?` :type Boolean))
  ;[1 0.7568 0] Interface
  (`self.PlayerGo_In` A B Pawn Speed `Rotate?`))

(event `/Game/Hide_easily/Blueprints/GameModeAndController/BI_HideEasilyControl.BI Update Hiding`
  (params (Bool :type Boolean))
  ;[1 0.7568 0] Interface
  (set `self.Hiding/Unhiding?` Bool))

(event `ShowScreenMessage`
  (params (`KillPlayer?` :type Boolean))
  (bind _ai_widget (`self.AI-Widget`))
  ;[0 1 0.25] AI Widget Interactions (Death and stuff)
  (if (not (`self.Dead?`))
    (`self.UpdateAI-Widget`)
    (if `KillPlayer?`
      (`self.Trigger Game Over Anims` null)
      (else
        (`KismetSystemLibrary.Delay` 2.0)
        (`/Engine/EditorBlueprintResources/StandardMacros.IsValid` _ai_widget
          (:`Is Valid`
            (`Widget.RemoveFromParent` _ai_widget)))))))

(event `/Game/Hide_easily/Blueprints/GameModeAndController/BI_HideEasilyControl.BI Add Hiding Place`
  (params (LookAtActor :type "Actor Object Reference"))
  ;[1 0.7568 0] Interface
  (`self.AddHidingPlace` LookAtActor))

(event `/Game/Hide_easily/Blueprints/GameModeAndController/BI_HideEasilyControl.BI Player Go Out`
  (params (A :type "Vector Structure") (B :type "Vector Structure") (Pawn :type "Actor Object Reference") (Speed :type "/Game/Hide_easily/Blueprints/GameModeAndController/E_HideSpeed Enum" :default "NewEnumerator0"))
  ;[1 0.7568 0] Interface
  (`self.PlayerGo_Out` A B Pawn Speed))

(event `/Game/Hide_easily/Blueprints/GameModeAndController/BI_HideEasilyControl.BI Player Go Under Bed`
  (params (Pawn :type "Actor Object Reference") (B :type "Vector Structure"))
  ;[1 0.7568 0] Interface
  (`self.PlayerGo_Under_Bed` Pawn B))

(event `/Game/Hide_easily/Blueprints/GameModeAndController/BI_HideEasilyControl.BI Rotate To Face Doors`
  (params (Pawn :type "Actor Object Reference") (Player :type "Vector Structure") (Target :type "Vector Structure"))
  ;[1 0.7568 0] Interface
  (`self.PlayerRotateToFaceDoors` Pawn Player Target))

(event `/Game/Hide_easily/Blueprints/GameModeAndController/BI_HideEasilyControl.BI Player Go Out Bed`
  (params (A :type "Vector Structure") (B :type "Vector Structure") (Pawn :type "Actor Object Reference"))
  ;[1 0.7568 0] Interface
  (`self.PlayerGo_Out_Bed` A B Pawn))

(event `/Game/Hide_easily/Blueprints/GameModeAndController/BI_HideEasilyControl.BI Pre Locate`
  (params (Pawn :type "Actor Object Reference") (A :type "Vector Structure") (B :type "Vector Structure"))
  ;[1 0.7568 0] Interface
  (`self.PreLocate` Pawn A B))

(event `/Game/Hide_easily/Blueprints/GameModeAndController/BI_HideEasilyControl.BI Change Control Rotation`
  (params (UsePawnControlRotation :type Boolean))
  ;[1 0.7568 0] Interface
  (`self.ChangeControlRotation` UsePawnControlRotation))

(event `PlayerGo_InRotate`
  (params (A :type "Vector Structure") (B :type "Vector Structure") (Pawn :type "Actor Object Reference") (Speed :type "/Game/Hide_easily/Blueprints/GameModeAndController/E_HideSpeed Enum" :default "NewEnumerator0"))
  (bind _relative_rotation (`self.Relative Rotation`))
  (bind _rootcomponent (`Actor.RootComponent` Pawn))
  ;[1 1 1] Go In/Rotate Go In
  ;;[0.9286 0.5318 1] enter the closet and ROTATE  // you call it inside Hide event RED
  (`/Game/PokeIsolationContent/Framework/Player/BP_PkO_Character.StopFootSteps` (`self.As BP Pk O Character`))
  (`self.SetHidingSpeed` Speed)
  (set `self.Relative Rotation` (`SceneComponent.K2_GetComponentRotation` _rootcomponent))
  (bind (_direction _track_0) (`Timeline|Timeline_7` :!via `PlayFromStart`)
    (:`Update`
      (`SceneComponent.K2_SetWorldLocation` _rootcomponent (`KismetMathLibrary.VLerp` A B _track_0) false true)
      (`self.SetControlRotation` (`self.GetInstigatorController` (cast `Pawn` Pawn :!pure true)) (`KismetMathLibrary.RLerp` _relative_rotation (`KismetMathLibrary.ComposeRotators` _relative_rotation (struct :`Yaw` 180.0)) _track_0 true)))
    (:`Finished`
      (`self.EnablePlayerInput`))))

(event `/Game/Hide_easily/Blueprints/GameModeAndController/BI_HideEasilyControl.BI You Are Dead`
  (params (`Kill player?` :type Boolean))
  ;[1 0.7568 0] Interface
  (`self.YouAreDead` `Kill player?`))

(event `/Game/Hide_easily/Blueprints/GameModeAndController/BI_HideEasilyControl.BI Show Interact Message Bed`
  (params (Bed :type "/Game/Hide_easily/Blueprints/BP_Bed Object Reference") (Bool :type Boolean))
  ;[1 0.7568 0] Interface
  (`self.ShowInteractMessageBed` Bed Bool))

(event `/Game/Hide_easily/Blueprints/GameModeAndController/BI_HideEasilyControl.BI Print Message`
  (params (Message :type String))
  ;[1 0.7568 0] Interface
  (`self.Print Message` Message))

(event `/Game/Hide_easily/Blueprints/GameModeAndController/BI_HideEasilyControl.BI Hide Interact Message Bed`
  (params (Bed :type "/Game/Hide_easily/Blueprints/BP_Bed Object Reference"))
  ;[1 0.7568 0] Interface
  (`self.HideInteractMessageBed` Bed))

(event `/Game/Hide_easily/Blueprints/GameModeAndController/BI_HideEasilyControl.BI Adjust After Hide`
  ;[1 0.7568 0] Interface
  (`self.AdjustsAfterHide`))

(event `/Game/Hide_easily/Blueprints/GameModeAndController/BI_HideEasilyControl.BI Hide Interact Message Book`
  (params (Book :type "/Game/Hide_easily/Blueprints/BP_Bookshelves Object Reference"))
  ;[1 0.7568 0] Interface
  (`self.HideInteractMessageBook` Book))

(event `/Game/Hide_easily/Blueprints/GameModeAndController/BI_HideEasilyControl.BI Adjust After Unhide`
  ;[1 0.7568 0] Interface
  (`self.AdjustsAfterUnhide`))

(event `/Game/Hide_easily/Blueprints/GameModeAndController/BI_HideEasilyControl.BI Show Interact Message Book`
  (params (Book :type "/Game/Hide_easily/Blueprints/BP_Bookshelves Object Reference") (`Hide/Unhide` :type Boolean))
  ;[1 0.7568 0] Interface
  (`self.ShowInteractMessageBook` Book `Hide/Unhide`))

(event `/Game/Hide_easily/Blueprints/GameModeAndController/BI_HideEasilyControl.BI Enable Rotation And Input`
  ;[1 0.7568 0] Interface
  (`self.EnableRotationAndInput`))

(event `Trigger Game Over Anims`
  (params (Haunter :type "Actor Object Reference"))
  (bind _returnvalue (`self.GetControlRotation`))
  (bind _as_bp_pk_o_character (`self.As BP Pk O Character`))
  (bind _returnvalue_2 (`self.K2_GetActorLocation` _as_bp_pk_o_character))
  ;[1 0.7369 0] Trigger Game Over and Haunter Anims
  (bind _asmonster_nbc (cast `/Game/MonsterAi_Kit/Monster_NBC` Haunter))
  (bind _output_get (set `self.As Monster NBC` _asmonster_nbc))
  (bind _asbp_pk_o_character (cast `/Game/PokeIsolationContent/Framework/Player/BP_PkO_Character` (`GameplayStatics.GetPlayerPawn` 0)))
  (bind _output_get_2 (set `self.As BP Pk O Character` _asbp_pk_o_character))
  (bind _returnvalue_3 (`self.Get Look At Rotation` (`self.K2_GetActorLocation` _output_get_2) (`SceneComponent.GetSocketLocation` (`Character.Mesh` _output_get) "WaistSocket") _returnvalue))
  (`self.DisableInput` (`GameplayStatics.GetPlayerPawn` 0) (`GameplayStatics.GetPlayerController` 0))
  (`/Game/PokeIsolationContent/Framework/Player/BP_PkO_Character.OnFlickerFlashLight` (`self.As BP Pk O Character`) true)
  (bind (_direction _lookat) (`Timeline|Smooth`)
    (:`Update`
      (`self.SetControlRotation` (`KismetMathLibrary.RLerp` _returnvalue _returnvalue_3 _lookat true))
      (message `/Game/Hide_easily/Blueprints/AI/BPI_TriggerAnims.TeleInFrontOfPlayer` _output_get _returnvalue_2 (`self.GetActorForwardVector` _as_bp_pk_o_character) 250.0 true))
    (:`Finished`
      (message `/Game/Hide_easily/Blueprints/AI/BPI_TriggerAnims.FoundPlayer` _output_get _returnvalue_2)
      (`/Game/PokeIsolationContent/Framework/Player/BP_PkO_Character.OnFlickerFlashLight` (`self.As BP Pk O Character`) false)
      (message `/Game/Hide_easily/Blueprints/AI/BPI_TriggerAnims.ScareAnim` _output_get)
      (`KismetSystemLibrary.K2_SetTimer` null "CheckIfGameOverScreenWorked" 2.0))))

(event `/Game/Hide_easily/Blueprints/GameModeAndController/BI_HideEasilyControl.BI Hide Interact Message Drawer`
  (params (Drawer :type "/Game/Hide_easily/Blueprints/Additional/BP_Drawer Object Reference"))
  ;[1 0.7568 0] Interface
  (`self.HideInteractMessageDrawer` Drawer))

(event `/Game/Hide_easily/Blueprints/GameModeAndController/BI_HideEasilyControl.BI Server Unhide Animation`
  ;[1 0.7568 0] Interface
  (`self.ServerUnhideAnimation`))

(event `/Game/Hide_easily/Blueprints/GameModeAndController/BI_HideEasilyControl.BI Server Hide Animation`
  ;[1 0.7568 0] Interface
  (`self.ServerHideAnimation`))

(event `/Game/Hide_easily/Blueprints/GameModeAndController/BI_HideEasilyControl.BI Show Interact Message Drawer`
  (params (Drawer :type "/Game/Hide_easily/Blueprints/Additional/BP_Drawer Object Reference") (Bool :type Boolean))
  ;[1 0.7568 0] Interface
  (`self.ShowInteractMessageDrawer` Drawer Bool))

(event `/Game/Hide_easily/Blueprints/GameModeAndController/BI_HideEasilyControl.BI Show Interact Message`
  (params (Closet :type "/Game/Hide_easily/Blueprints/BP_Closet_1 Object Reference") (Bool :type Boolean))
  ;[1 0.7568 0] Interface
  (`self.ShowInteractMessage` Closet Bool))

(event `/Game/Hide_easily/Blueprints/GameModeAndController/BI_HideEasilyControl.BI Enable Player Input`
  ;[1 0.7568 0] Interface
  (`self.EnablePlayerInput`))

(event `/Game/Hide_easily/Blueprints/GameModeAndController/BI_HideEasilyControl.BI Disable Player Input`
  ;[1 0.7568 0] Interface
  (`self.DisablePlayerInput`))

(event `/Game/Hide_easily/Blueprints/GameModeAndController/BI_HideEasilyControl.BI Hide Interact Message`
  (params (Closet :type "/Game/Hide_easily/Blueprints/BP_Closet_1 Object Reference"))
  ;[1 0.7568 0] Interface
  (`self.HideInteractMessage` Closet))

(event `CheckIfGameOverScreenWorked`
  (if (not (`self.bGameOver`))
    (`self.Show Game Over Screen`)))

(event `Show Game Over Screen`
  ;[1 0.07651 0] Show Game Over Screen
  (set `self.bGameOver` true)
  (bind _returnvalue (`|CreateWidget` "/Game/PokeIsolationContent/Widgets/W_GameOverScreen.W_GameOverScreen_C"))
  (`UserWidget.AddToViewport` _returnvalue 0)
  (`KismetSystemLibrary.Delay` 2.0)
  (`GameplayStatics.SetGamePaused` true)
  (`WidgetBlueprintLibrary.SetInputMode_UIOnlyEx` (`GameplayStatics.GetPlayerController` 0) _returnvalue)
  (set `PlayerController.bShowMouseCursor` true (`GameplayStatics.GetPlayerController` 0)))

(event `Show Game Win Screen`
  ;[0 1 0.06008] Game Win Screen
  (`self.DisableInput` (`GameplayStatics.GetPlayerPawn` 0) (`GameplayStatics.GetPlayerController` 0))
  (`GameplayStatics.PlaySound2D` null 1.0 1.0 0.0 null null)
  (bind _returnvalue (`|CreateWidget` "/Game/PokeIsolationContent/Widgets/W_GameWinScreen.W_GameWinScreen_C"))
  (`UserWidget.AddToViewport` _returnvalue 0)
  (`GameplayStatics.SetGamePaused` true)
  (`WidgetBlueprintLibrary.SetInputMode_UIOnlyEx` (`GameplayStatics.GetPlayerController` 0) null)
  (set `PlayerController.bShowMouseCursor` true (`GameplayStatics.GetPlayerController` 0)))

(fn `AddHidingPlace`
  (params (LookAtActor :type "Actor Object Reference"))
  (`self.RemoveLast`)
  (set `self.Look at Actor` LookAtActor))

(fn `BI Get Dead`
  (returns (Dead :type Boolean))
  (return (`self.Dead?`)))

(fn `BI Get Hiding/Unhiding`
  (returns (`Hiding/Unhiding` :type Boolean))
  (return (`self.Hiding/Unhiding?`)))

(fn `Get Look At Rotation`
  (params (Player :type "Vector Structure") (Target :type "Vector Structure") (PlayerRotation :type "Rotator Structure"))
  (returns (ReturnValue :type "Rotator Structure"))
  (return (`KismetMathLibrary.MakeRotator` (.roll (`KismetMathLibrary.FindLookAtRotation` Player Target)) (/ (.pitch (`KismetMathLibrary.FindLookAtRotation` Player Target)) 4.0) (.yaw (`KismetMathLibrary.FindLookAtRotation` Player Target)))))

(fn `GetMidLocation`
  (params (Start :type "Vector Structure") (End :type "Vector Structure") (Alpha :type "Float (double-precision)"))
  (returns (ReturnValue :type "Vector Structure"))
  (return (`KismetMathLibrary.MakeVector` (.x (`KismetMathLibrary.VLerp` Start End Alpha)) (.y (`KismetMathLibrary.VLerp` Start End Alpha)) (.z Start))))

(fn `RemoveLast`
  (bind _look_at_actor (`self.Look at Actor`))
  (bind _asbi_hide_easily_control (cast `/Game/Hide_easily/Blueprints/GameModeAndController/BI_HideEasilyControl` self :!pure true))
  (`/Engine/EditorBlueprintResources/StandardMacros.IsValid` _look_at_actor
    (:`Is Valid`
      (bind _asbp_closet_1 (cast `/Game/Hide_easily/Blueprints/BP_Closet_1` _look_at_actor)
        (:`then`
          (`/Game/Hide_easily/Blueprints/BP_Closet_1.Server_Hide_Message` _asbp_closet_1 _asbi_hide_easily_control))
        (:`CastFailed`
          (bind _asbp_bed (cast `/Game/Hide_easily/Blueprints/BP_Bed` _look_at_actor)
            (:`then`
              (`/Game/Hide_easily/Blueprints/BP_Bed.Server_Hide_Message` _asbp_bed _asbi_hide_easily_control))
            (:`CastFailed`
              (bind _asbp_bookshelves (cast `/Game/Hide_easily/Blueprints/BP_Bookshelves` _look_at_actor)
                (:`then`
                  (`/Game/Hide_easily/Blueprints/BP_Bookshelves.Server_Hide_Message` _asbp_bookshelves _asbi_hide_easily_control))
                (:`CastFailed`
                  (bind _asbp_drawer (cast `/Game/Hide_easily/Blueprints/Additional/BP_Drawer` _look_at_actor))
                  (`/Game/Hide_easily/Blueprints/Additional/BP_Drawer.Server_Hide_Message` _asbp_drawer _asbi_hide_easily_control))))))))))

(fn `SetHidingSpeed`
  (params (Index :type "/Game/Hide_easily/Blueprints/GameModeAndController/E_HideSpeed Enum" :default "NewEnumerator0"))
  (bind _goinclosettimer (`self.GoInClosetTimer`))
  (`TimelineComponent.SetTimelineLength` _goinclosettimer (select `/Game/Hide_easily/Blueprints/GameModeAndController/E_HideSpeed` Index :`NewEnumerator0` 1.0 :`NewEnumerator1` 0.8))
  (`TimelineComponent.SetFloatCurve` _goinclosettimer (select `/Game/Hide_easily/Blueprints/GameModeAndController/E_HideSpeed` Index :`NewEnumerator0` "/Game/Hide_easily/Curves/C_One.C_One" :`NewEnumerator1` "/Game/Hide_easily/Curves/C_Point8.C_Point8" :!type "CurveFloat Object Reference") "Track_0"))

(fn `SetUnhidingSpeed`
  (params (Index :type "/Game/Hide_easily/Blueprints/GameModeAndController/E_HideSpeed Enum" :default "NewEnumerator0"))
  (bind _gooutclosettimer (`self.GoOutClosetTimer`))
  (`TimelineComponent.SetTimelineLength` _gooutclosettimer (select `/Game/Hide_easily/Blueprints/GameModeAndController/E_HideSpeed` Index :`NewEnumerator0` 1.0 :`NewEnumerator1` 0.8))
  (`TimelineComponent.SetFloatCurve` _gooutclosettimer (select `/Game/Hide_easily/Blueprints/GameModeAndController/E_HideSpeed` Index :`NewEnumerator0` "/Game/Hide_easily/Curves/C_One.C_One" :`NewEnumerator1` "/Game/Hide_easily/Curves/C_Point8.C_Point8" :!type "CurveFloat Object Reference") "Track_0"))

(fn `UpdateAI-Widget`
  (`/Engine/EditorBlueprintResources/StandardMacros.IsValid` (`self.AI-Widget`)
    (:`Is Valid`
      (`Widget.RemoveFromParent` (`self.AI-Widget`))
      (set `self.AI-Widget` null))))

(fn `UserConstructionScript`)