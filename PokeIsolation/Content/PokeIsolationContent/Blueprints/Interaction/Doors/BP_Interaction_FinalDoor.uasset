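; Final mansion exit door that unlocks when the interacting player's puzzle piece count matches the required amount, triggering the win screen.
; Otherwise it plays a locked sound and prints a hint.
; Once unlocked, interaction toggles a timeline-driven yaw swing, reversed to close, with open direction taken from the player's direction factor.
; A passthrough trigger fires an event dispatcher and an empty Passthrough hook when the player overlaps it.
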(event `/Game/PokeIsolationContent/Blueprints/Interaction/BPI_Interaction.OnInteract`
  (params (Player :type "Character Object Reference"))
  (bind (_returnvalue_roll _returnvalue_pitch _returnvalue_yaw) (`KismetMathLibrary.BreakRotator` (`SceneComponent.K2_GetComponentRotation` (`self.Arrow`))))
  (bind (_returnvalue_roll_2 _returnvalue_pitch_2 _returnvalue_yaw_2) (`KismetMathLibrary.BreakRotator` (`SceneComponent.K2_GetComponentRotation` (`/Game/FirstPerson/Blueprints/BP_FirstPersonCharacter.FirstPersonCamera` (`self.PlayerUsingDoor`)))))
  (if (`self.bIsLocked`)
    ;[0.04668 0.1198 0] Check if Player Has All Puzzle Pieces
    (bind _asbp_pk_o_character (cast `/Game/PokeIsolationContent/Framework/Player/BP_PkO_Character` Player))
    (set `self.PlayerUsingDoor` _asbp_pk_o_character)
    (if (== (`/Game/PokeIsolationContent/Framework/Player/BP_PkO_Character.CollectedPuzzleCount` _asbp_pk_o_character) (`self.AmountOfPuzzlePiecesNeeded`))
      (bind _asbp_pk_o_player_controller (cast `/Game/PokeIsolationContent/Blueprints/GameModeandController/BP_PkO_PlayerController` (`GameplayStatics.GetPlayerController` 0)))
      (`/Game/PokeIsolationContent/Blueprints/GameModeandController/BP_PkO_PlayerController.Show Game Win Screen` _asbp_pk_o_player_controller)
      (`KismetSystemLibrary.PrintString` (`KismetTextLibrary.Conv_TextToString` (`|FormatText` "Congratulations! You escaped the mansion!")))
      (set `self.bIsLocked` false)
      (if (`self.bIsOpen`) :!label _label
        (`self.CloseDoor` 1.0)
        (else
          (`self.OpenDoor` 1.0 (* (`KismetMathLibrary.SelectFloat` 1.0 -1.0 (`KismetMathLibrary.InRange_FloatFloat` (- (+ (`KismetMathLibrary.NormalizeAxis` _returnvalue_yaw) 180.0) (+ (`KismetMathLibrary.NormalizeAxis` _returnvalue_yaw_2) 180.0)) -90.0 90.0 false false)) (`self.MaxRotation`)))))
      (else
        ;[1 1 1] Door locked sfx
        (`GameplayStatics.PlaySoundAtLocation` "/Game/Sounds/Doors/SC_DoorLocked.SC_DoorLocked" (`self.OpenCloseSoundLocation`) (struct) 0.7 1.0 0.0 null null null null)
        (`KismetSystemLibrary.PrintString` (`KismetTextLibrary.Conv_TextToString` (`|FormatText` "Door needs all three pieces of the puzzle to open.")))
        (set `self.PlayerUsingDoor` null)))
    (else
      (bind _asbp_pk_o_character_2 (cast `/Game/PokeIsolationContent/Framework/Player/BP_PkO_Character` Player))
      (set `self.PlayerUsingDoor` _asbp_pk_o_character_2)
      (if (`self.bCanSwitchState`)
        (goto _label)))))

(event `OpenDoor`
  (params (Rate :type "Float (double-precision)" :default 1.0) (DirectionFactor :type "Float (double-precision)" :default 1.0))
  (bind _doorrotationroot (`self.DoorRotationRoot`))
  (bind (_relativerotation_roll _relativerotation_pitch) (`KismetMathLibrary.BreakRotator` (`SceneComponent.RelativeRotation` _doorrotationroot)))
  ;[1 1 1] Door State Switch
  (`self.PlayOpenSound`)
  (set `self.bIsOpen` true)
  (set `self.RotationFactor` DirectionFactor)
  (`TimelineComponent.SetPlayRate` (`self.SwitchState`) Rate)
  (bind (_direction _tl_doormovement) (`Timeline|SwitchState` :!label _label_2)
    (:`Update`
      (set `self.bCanSwitchState` false)
      (`SceneComponent.K2_SetRelativeRotation` _doorrotationroot (`KismetMathLibrary.MakeRotator` _relativerotation_roll _relativerotation_pitch (`KismetMathLibrary.Lerp` 0.0 (`self.RotationFactor`) _tl_doormovement)) false false))
    (:`Finished`
      (set `self.bCanSwitchState` true)
      (set `self.PlayerUsingDoor` null)
      (`TimelineComponent.SetPlayRate` (`self.SwitchState`) 1.0))))

(event `CloseDoor`
  (params (Rate :type "Float (double-precision)" :default 1.0))
  ;[1 1 1] Door State Switch
  (`self.PlayCloseSound`)
  (set `self.bIsOpen` false)
  (`TimelineComponent.SetPlayRate` (`self.SwitchState`) Rate)
  (goto _label_2 :!via `Reverse`))

(event `self.PassthroughEventTrigger.OnComponentBeginOverlap`
  (params (OverlappedComponent :type "PrimitiveComponent Object Reference") (OtherActor :type "Actor Object Reference") (OtherComp :type "PrimitiveComponent Object Reference") (OtherBodyIndex :type Integer) (bFromSweep :type Boolean) (SweepResult :type "HitResult Structure (by ref)"))
  (cast `/Game/PokeIsolationContent/Framework/Player/BP_PkO_Character` OtherActor)
  (`self.OnPassthroughEvent`)
  (`self.Passthrough`))

(fn `OpenCloseSoundLocation`
  (returns (ReturnValue :type "Vector Structure"))
  (bind _door (`self.Door`))
  (return (+ (`SceneComponent.K2_GetComponentLocation` _door) (* (`SceneComponent.GetForwardVector` _door) -30.0))))

(fn `Passthrough`)

(fn `PlayCloseSound`
  (`GameplayStatics.PlaySoundAtLocation` "/Game/Sounds/Doors/SC_DoorClose.SC_DoorClose" (`self.OpenCloseSoundLocation`) (struct) 0.1 1.0 0.0 null null null null))

(fn `PlayOpenSound`
  (`GameplayStatics.PlaySoundAtLocation` "/Game/Sounds/Doors/SC_DoorOpen.SC_DoorOpen" (`self.OpenCloseSoundLocation`) (struct) 0.3 1.0 0.0 null null null null))

(fn `UserConstructionScript`)