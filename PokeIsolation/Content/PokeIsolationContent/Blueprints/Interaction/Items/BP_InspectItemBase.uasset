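; Base Blueprint for an inspectable item that flies from its place in the world to the player character's inspect point.
; OnInteract turns off mesh physics and collision, shows the HUD inspect widget with the item's details, and plays a timeline that interpolates the transform.
; Inspect_PutAway clears the widget and reverses the timeline, restoring collision and physics when it finishes.
; Collectable items also enable player input during travel, though no input handling is defined here.
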(event `self.ReceiveBeginPlay`)

(event `/Game/PokeIsolationContent/Blueprints/Interaction/BPI_Interaction.OnInteract`
  (params (Player :type "Character Object Reference"))
  (`PrimitiveComponent.SetSimulatePhysics` (`self.Mesh`) false)
  (`PrimitiveComponent.SetCollisionEnabled` (`self.Mesh`) "NoCollision")
  (set `self.InitialTransform` (`SceneComponent.K2_GetComponentToWorld` (`self.Mesh`)))
  (bind _asbp_pk_o_character (cast `/Game/PokeIsolationContent/Framework/Player/BP_PkO_Character` Player))
  (bind _asbp_pko_hud (cast `/Game/PokeIsolationContent/Framework/HUD/BP_PKO_HUD` (`PlayerController.GetHUD` (`GameplayStatics.GetPlayerController` 0))))
  (`/Game/PokeIsolationContent/Framework/HUD/BP_PKO_HUD.ShowHideInspectWidget` _asbp_pko_hud (`self.Name`) (`self.Description`) (`self.bCollectable`))
  (bind (_direction _interactioninterp) (`Timeline|TravelTimeline` :!label _label)
    (:`Update`
      (bind _inspectpoint (`/Game/PokeIsolationContent/Framework/Player/BP_PkO_Character.InspectPoint` _asbp_pk_o_character))
      (`SceneComponent.K2_SetWorldLocationAndRotation` (`self.Mesh`) (`KismetMathLibrary.VLerp` (.location (`self.InitialTransform`)) (`SceneComponent.K2_GetComponentLocation` _inspectpoint) _interactioninterp) (`KismetMathLibrary.RLerp` (.rotation (`self.InitialTransform`)) (select `ETimelineDirection` _direction :`Forward` (`SceneComponent.K2_GetComponentRotation` _inspectpoint) :`Backward` (`SceneComponent.K2_GetComponentRotation` (`self.Mesh`))) _interactioninterp true) false false)
      (if (`self.bCollectable`)
        (`self.EnableInput` (`GameplayStatics.GetPlayerController` 0))))
    (:`Finished`
      (switch `ETimelineDirection` _direction
        (:`Backward`
          (`PrimitiveComponent.SetCollisionEnabled` (`self.Mesh`) "QueryAndPhysics")
          (`PrimitiveComponent.SetSimulatePhysics` (`self.Mesh`) true))))))

(event `Inspect_PutAway`
  (`/Game/PokeIsolationContent/Framework/HUD/BP_PKO_HUD.ShowHideInspectWidget` (stale `/Game/PokeIsolationContent/Blueprints/Interaction/BPI_Interaction.OnInteract` _asbp_pko_hud) "" "" false)
  (goto _label :!via `Reverse`))

(fn `UserConstructionScript`)