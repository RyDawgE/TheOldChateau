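; Spawns and manages Monster_GastlyAi enemies at BP_GastlySpawnPoint actors, either at every point or up to MaxGastlys at random ones.
; Each death starts a timer that respawns a Gastly at its reported location, tracked through a map and dead list.
; Gastly time events feed a counter that broadcasts CallDad with the player's location at a threshold.
; Event bindings are made only at BeginPlay, so respawned Gastlys are not bound.
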(event `self.ReceiveBeginPlay`
  (`|ExecutionSequence`
    (:`then_0`
      (bind _outactors (`GameplayStatics.GetAllActorsOfClass` "/Game/PokeIsolationContent/Blueprints/ItemSpawning/BP_GastlySpawnPoint.BP_GastlySpawnPoint_C"))
      (for _array_element _outactors
        (`KismetArrayLibrary.Array_Add` (`self.SpawnLocations`) _array_element))
      (bind _asbp_pk_o_character (cast `/Game/PokeIsolationContent/Framework/Player/BP_PkO_Character` (`GameplayStatics.GetPlayerCharacter` 0)))
      (set `self.As BP Pk O Character` _asbp_pk_o_character)
      (if (`self.RandomSpawn?`)
        (`self.Spawn Gastlys`)
        (else
          (for _array_element_2 (`self.SpawnLocations`)
            (bind _returnvalue (`|SpawnActorFromClass` :`Class` "/Game/MonsterAi_Kit/Monster_GastlyAi.Monster_GastlyAi_C" :`SpawnTransform` (`KismetMathLibrary.Conv_VectorToTransform` (`self.K2_GetActorLocation` _array_element_2)) :`CollisionHandlingOverride` "Undefined" :`TransformScaleMethod` "MultiplyWithRoot" :`FleeSounds` (`self.GastlyFleeSounds`) :`SlowPlayerSpeedTo` (`self.SlowAmount`) :`FleeDuration` (`self.Flee Duration`) :`PatrolSplinePath` null :`DieRagDoll?` false :`SpeedVariables` (`self.Speed Variables`) :`DamageEffect` "/Game/MonsterAi_Kit/BloodFX/P_Blood.P_Blood" :`CanKill?` false :`Instigator` null))
            (`/Engine/EditorBlueprintResources/StandardMacros.IsValid` _returnvalue
              (:`Is Valid`
                (`KismetArrayLibrary.Array_Add` (`self.ListOfActiveGastlys`) _returnvalue)
                (`KismetSystemLibrary.Delay` 2.0))))
          (`KismetSystemLibrary.PrintString` (`KismetTextLibrary.Conv_TextToString` (`|FormatText` "{number} gastlys were spawned" (`KismetArrayLibrary.Array_Length` (`self.ListOfActiveGastlys`)))) true true (struct :`G` 0.66 :`B` 1.0 :`A` 1.0) 10.0)))
      (for _array_element_3 (`self.ListOfActiveGastlys`)
        (add `/Game/MonsterAi_Kit/Monster_GastlyAi.OnGastlyHasDied` _array_element_3 (delegate `OnGastlyHasDied`))
        (add `/Game/MonsterAi_Kit/Monster_GastlyAi.OnIncrementTime` _array_element_3 (delegate `TimeTillCallDad`))))))

(event `TimeTillCallDad`
  (bind _result (`/Engine/EditorBlueprintResources/StandardMacros.IncrementFloat` (`self.AccumulatedTime`))
    (:`  `
      (if (>= _result (`self.Call Daddy At This Time`))
        (`self.Call Dad` (`self.K2_GetActorLocation` (`self.As BP Pk O Character`)))
        (set `self.AccumulatedTime` 0.0)))))

(event `OnGastlyHasDied`
  (params (GastlyThatHasDied :type "/Game/MonsterAi_Kit/Monster_GastlyAi Object Reference") (RespawnLocation :type "Vector Structure"))
  (`KismetArrayLibrary.Array_RemoveItem` (`self.ListOfActiveGastlys`) GastlyThatHasDied)
  (bind _returnvalue (`KismetSystemLibrary.K2_SetTimerDelegate` (delegate `TriggerRespawnOfGastly`) (`self.RespawnTime`)))
  (`BlueprintMapLibrary.Map_Add` (`self.RespawnGastlyMap`) GastlyThatHasDied (make `/Game/MonsterAi_Kit/ST_GastlyRespawnInfo` RespawnLocation _returnvalue))
  (`KismetArrayLibrary.Array_Add` (`self.ListOfDeadGastlys`) GastlyThatHasDied))

(event `Respawn Gastlys`
  (params (InLocation :type "Vector Structure"))
  (bind _returnvalue (`|SpawnActorFromClass` :`Class` "/Game/MonsterAi_Kit/Monster_GastlyAi.Monster_GastlyAi_C" :`SpawnTransform` (`KismetMathLibrary.Conv_VectorToTransform` InLocation) :`CollisionHandlingOverride` "Undefined" :`TransformScaleMethod` "MultiplyWithRoot" :`FleeSounds` (`self.GastlyFleeSounds`) :`SlowPlayerSpeedTo` (`self.SlowAmount`) :`Duration` (`self.SlowDuration`) :`FleeDuration` (`self.Flee Duration`) :`PatrolSplinePath` null :`DieRagDoll?` false :`SpeedVariables` (`self.Speed Variables`) :`DamageEffect` "/Game/MonsterAi_Kit/BloodFX/P_Blood.P_Blood" :`CanKill?` false :`Instigator` null))
  (`KismetArrayLibrary.Array_Add` (`self.ListOfActiveGastlys`) _returnvalue)
  (`KismetSystemLibrary.PrintString` "Gastly respawned" true true (struct :`R` 1.0 :`B` 0.667799 :`A` 1.0) 10.0))

(event `TriggerRespawnOfGastly`
  (for _array_element (`self.ListOfDeadGastlys`)
    (bind (_value _returnvalue) (`BlueprintMapLibrary.Map_Find` (`self.RespawnGastlyMap`) _array_element))
    (if (and _returnvalue (== (`KismetSystemLibrary.K2_GetTimerRemainingTimeHandle` (`.RespawnTimer_6_7AE1A13844EAE85B2B6E958F9DF62DCD` (break `/Game/MonsterAi_Kit/ST_GastlyRespawnInfo` _value))) 0.0))
      (`KismetSystemLibrary.K2_ClearAndInvalidateTimerHandle` (`.RespawnTimer_6_7AE1A13844EAE85B2B6E958F9DF62DCD` (break `/Game/MonsterAi_Kit/ST_GastlyRespawnInfo` _value)))
      (`self.Respawn Gastlys` (break `/Game/MonsterAi_Kit/ST_GastlyRespawnInfo` _value))
      (`BlueprintMapLibrary.Map_Remove` (`self.RespawnGastlyMap`) _array_element)
      (`KismetArrayLibrary.Array_RemoveItem` (`self.ListOfDeadGastlys`) _array_element))))

(event `Spawn Gastlys 2`
  (bind _outitem (`KismetArrayLibrary.Array_Random` (`self.UnusedSpawnPoints`)))
  (set `self.UnusedSpawnPoints` (`self.SpawnLocations`))
  (if (and (< (`self.LoopCounter`) (`self.MaxGastlys`)) (> (`KismetArrayLibrary.Array_Length` (`self.UnusedSpawnPoints`)) 0)) :!label _label
    (bind _returnvalue (`|SpawnActorFromClass` :`Class` "/Game/MonsterAi_Kit/Monster_GastlyAi.Monster_GastlyAi_C" :`SpawnTransform` (`KismetMathLibrary.Conv_VectorToTransform` (`self.K2_GetActorLocation` _outitem)) :`CollisionHandlingOverride` "Undefined" :`TransformScaleMethod` "MultiplyWithRoot" :`FleeSounds` (`self.GastlyFleeSounds`) :`FleeDuration` (`self.Flee Duration`) :`PatrolSplinePath` null :`DieRagDoll?` false :`SpeedVariables` (`self.Speed Variables`) :`DamageEffect` "/Game/MonsterAi_Kit/BloodFX/P_Blood.P_Blood" :`CanKill?` false :`Instigator` null))
    (`KismetArrayLibrary.Array_RemoveItem` (`self.UnusedSpawnPoints`) _outitem)
    (`KismetArrayLibrary.Array_Add` (`self.ListOfActiveGastlys`) _returnvalue)
    (`/Engine/EditorBlueprintResources/StandardMacros.IncrementInt` (`self.LoopCounter`)
      (:`  `
        (`KismetSystemLibrary.Delay` 0.2)
        (goto _label)))
    (else
      (`KismetSystemLibrary.PrintString` (`KismetTextLibrary.Conv_TextToString` (`|FormatText` "{number} gastlys were spawned" (`self.LoopCounter`))) true true (struct :`G` 0.66 :`B` 1.0 :`A` 1.0) 10.0))))

(fn `Remove Gastly from List Of Active`
  (params (GastlyThatHasDied :type "Actor Object Reference (by ref)")))

(fn `Spawn Gastlys`
  (returns (MaxGastlysSpawned :type Boolean))
  (locals (UnusedSpawnPoints :type "Array of /Game/PokeIsolationContent/Blueprints/ItemSpawning/BP_GastlySpawnPoint Object Reference") (LoopCounter :type Integer))
  (bind _outitem (`KismetArrayLibrary.Array_Random` (`local.UnusedSpawnPoints`)))
  (set `local.UnusedSpawnPoints` (`self.SpawnLocations`))
  (if (and (< (`local.LoopCounter`) (`self.MaxGastlys`)) (> (`KismetArrayLibrary.Array_Length` (`local.UnusedSpawnPoints`)) 0)) :!label _label
    (bind _returnvalue (`|SpawnActorFromClass` :`Class` "/Game/MonsterAi_Kit/Monster_GastlyAi.Monster_GastlyAi_C" :`SpawnTransform` (`KismetMathLibrary.Conv_VectorToTransform` (`self.K2_GetActorLocation` _outitem)) :`CollisionHandlingOverride` "Undefined" :`TransformScaleMethod` "MultiplyWithRoot" :`FleeSounds` (`self.GastlyFleeSounds`) :`SlowPlayerSpeedTo` (`self.SlowAmount`) :`Duration` (`self.SlowDuration`) :`FleeDuration` (`self.Flee Duration`) :`PatrolSplinePath` null :`DieRagDoll?` false :`SpeedVariables` (`self.Speed Variables`) :`DamageEffect` "/Game/MonsterAi_Kit/BloodFX/P_Blood.P_Blood" :`CanKill?` false :`Instigator` null))
    (`KismetArrayLibrary.Array_RemoveItem` (`local.UnusedSpawnPoints`) _outitem)
    (`KismetArrayLibrary.Array_Add` (`self.ListOfActiveGastlys`) _returnvalue)
    (`/Engine/EditorBlueprintResources/StandardMacros.IncrementInt` (`local.LoopCounter`)
      (:`  `
        (goto _label)))
    (else
      (`KismetSystemLibrary.PrintString` (`KismetTextLibrary.Conv_TextToString` (`|FormatText` "{number} gastlys were spawned" (`local.LoopCounter`))) true true (struct :`G` 0.66 :`B` 1.0 :`A` 1.0) 10.0)
      (return false))))

(fn `UserConstructionScript`)