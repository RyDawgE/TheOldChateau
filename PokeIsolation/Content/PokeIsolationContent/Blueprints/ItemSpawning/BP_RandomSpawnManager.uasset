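; BP_RandomSpawnManager spawns a configured list of items at random spawnpoints when play begins.
; It gathers unique BP_C_SpawnpointComponents from the actors in ActorsWithSpawnpoints into one pool.
; Each item ID is looked up in DT_Items, and its actor class is spawned, attached to a spawnpoint keeping world transform.
; Random is pure and re-evaluates per step, so the spawn, attach and pool removal can hit different spawnpoints.
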(event `self.ReceiveBeginPlay`
  (bind _outitem (`KismetArrayLibrary.Array_Random` (`self.AllSpawnpoints`)))
  (for _array_element (`self.ActorsWithSpawnpoints`)
    (for _array_element_2 (`self.K2_GetComponentsByClass` _array_element "/Game/PokeIsolationContent/Blueprints/ItemSpawning/BP_C_SpawnpointComponent.BP_C_SpawnpointComponent_C")
      (`KismetArrayLibrary.Array_AddUnique` (`self.AllSpawnpoints`) _array_element_2)))
  (for _array_element_3 (`self.ItemIDs`)
    (bind _returnvalue (`|GetDataTableRow` "/Game/PokeIsolationContent/Blueprints/ItemSpawning/DT_Items.DT_Items" _array_element_3)
      (:`then`
        (bind _returnvalue_2 (`|SpawnActorFromClass` (`.ActorClass_3_308A4B4944911C680D291B8F4337D82F` (break `/Game/PokeIsolationContent/Blueprints/ItemSpawning/S_DT_Item` _returnvalue)) (`KismetMathLibrary.MakeTransform` (`SceneComponent.K2_GetComponentLocation` _outitem) (`SceneComponent.K2_GetComponentRotation` _outitem)) "AlwaysSpawn" "MultiplyWithRoot" null null))
        (`self.K2_AttachToComponent` _returnvalue_2 _outitem "None" "KeepWorld" "KeepWorld" "KeepWorld" true)
        (`KismetArrayLibrary.Array_RemoveItem` (`self.AllSpawnpoints`) _outitem)))))

(fn `UserConstructionScript`)