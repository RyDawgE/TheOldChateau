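; BP_EscapeTheMansion re-arms every Haunter patrol-change trigger box when the player character signals the Escape the Mansion event.
; On BeginPlay it binds its reset handler to that event on BP_PkO_Character and caches all BP_HaunterPatrolChange actors in the level.
; The handler sets each cached box active, calls its ResetTriggerBox and prints an on-screen confirmation; this Blueprint has no overlap logic of its own.
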(event `self.ReceiveBeginPlay`
  (`|ExecutionSequence`
    (:`then_0`
      (bind _asbp_pk_o_character (cast `/Game/PokeIsolationContent/Framework/Player/BP_PkO_Character` (`GameplayStatics.GetPlayerCharacter` 0)))
      (add `/Game/PokeIsolationContent/Framework/Player/BP_PkO_Character.EscapeTheMansion` _asbp_pk_o_character (delegate `ResetAllTriggerBoxes`)))
    (:`then_1`
      (bind _outactors (`GameplayStatics.GetAllActorsOfClass` "/Game/PokeIsolationContent/Blueprints/TriggerBoxes/BP_HaunterPatrolChange.BP_HaunterPatrolChange_C"))
      (set `self.ArrayOfPatrolTriggerBoxes` _outactors))))

(event `ResetAllTriggerBoxes`
  (for _array_element (`self.ArrayOfPatrolTriggerBoxes`)
    (set `/Game/PokeIsolationContent/Blueprints/TriggerBoxes/BP_HaunterPatrolChange.Active` true _array_element)
    (`/Game/PokeIsolationContent/Blueprints/TriggerBoxes/BP_HaunterPatrolChange.Reset Trigger Box` _array_element))
  (`KismetSystemLibrary.PrintString` "Escape the Mansion: All Haunter Trigger Boxes Have Been Reset" true true (struct :`R` 1.0 :`B` 0.171393 :`A` 1.0) 20.0))

(fn `UserConstructionScript`)