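; Trigger box that fires a one-time Haunter jump scare when the player overlaps it.
; BeginPlay caches the monster tagged "Haunter"; the overlap plays its montage and, given a spawn actor and no particle effect, teleports it there facing the player.
; It then plays a scare sound, applies scary face, speed buffs and patrol settings, and sends it toward the player.
; It also updates Haunter's spawn point and can choose a patrol path by floor.
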(event `self.ReceiveBeginPlay`
  ;[0.06771 0.06771 0.06771] Get and Save Haunter in Map WIll need to be ran again if Haunter is destroyed for some reason
  (bind _outactors (`GameplayStatics.GetAllActorsWithTag` "Haunter"))
  (bind _asmonster_nbc (cast `/Game/MonsterAi_Kit/Monster_NBC` (`|GetArrayItem` _outactors)))
  (set `self.Haunter` _asmonster_nbc))

(event `self.Box.OnComponentBeginOverlap`
  (params (OverlappedComponent :type "PrimitiveComponent Object Reference") (OtherActor :type "Actor Object Reference") (OtherComp :type "PrimitiveComponent Object Reference") (OtherBodyIndex :type Integer) (bFromSweep :type Boolean) (SweepResult :type "HitResult Structure (by ref)"))
  (bind _where_the_ai_spawns (`self.Where the Ai Spawns`))
  (bind _haunter (`self.Haunter`))
  (bind (_returnvalue_x _returnvalue_y _returnvalue_z) (`KismetMathLibrary.BreakVector` (`self.K2_GetActorLocation` _where_the_ai_spawns)))
  (bind _asbp_pk_o_character (cast `/Game/PokeIsolationContent/Framework/Player/BP_PkO_Character` OtherActor))
  (`/Engine/EditorBlueprintResources/StandardMacros.DoOnce` false
    (:`Completed`
      (`/Game/MonsterAi_Kit/Monster_NBC.PlayMontage` (`self.Haunter`) (`self.Montage to Play`) (`self.Play Rate`) (`self.Starting Position`) (`self.Starting Section`))
      (`/Engine/EditorBlueprintResources/StandardMacros.IsValid` _where_the_ai_spawns
        (:`Is Valid`
          (`/Engine/EditorBlueprintResources/StandardMacros.IsValid` (`self.ParticleEffect`)
            (:`Is Not Valid`
              (set `/Game/MonsterAi_Kit/Monster_NBC.HaunterLocation` (`self.LocationOfThisBox`) (`self.Haunter`))
              (`/Game/MonsterAi_Kit/Monster_NBC.Set Scary Face` _haunter)
              (`self.K2_SetActorLocationAndRotation` (`self.Haunter`) (`KismetMathLibrary.MakeVector` _returnvalue_x _returnvalue_y (+ _returnvalue_z 100.0)) (`KismetMathLibrary.FindLookAtRotation` (`self.K2_GetActorLocation` _where_the_ai_spawns) (`self.K2_GetActorLocation` _asbp_pk_o_character)) false false)
              (`GameplayStatics.PlaySoundAtLocation` (`self.ScareSound`) (`self.K2_GetActorLocation` _asbp_pk_o_character) (struct) 0.7 1.0 2.0 null null null null)
              (`/Game/MonsterAi_Kit/Monster_NBC.Jump Scare Buffs` _haunter (`self.Patrol State Speed`) (`self.Chase Speed`) (`self.Duration`) 0.0)
              (`/Game/MonsterAi_Kit/Monster_NBC.Set Patrol Details` (`self.Haunter`) (`self.New Patrol Path`) (`self.Patrol Looping?`) (`self.Return to Spawn Point?`))
              (`AITask_MoveTo.AIMoveTo` (`AIBlueprintHelperLibrary.GetAIController` (`self.Haunter`)) (`self.K2_GetActorLocation` _asbp_pk_o_character) _asbp_pk_o_character -1.0 "Default" "Default" true false
                (:`then`
                  (set `/Game/MonsterAi_Kit/Monster_NBC.spawnPoint` (`self.K2_GetActorLocation` (`self.Where the Ai Spawns`)) (`self.Haunter`))
                  (if (`self.RandomPatrolPathByFloor`)
                    (`/Game/MonsterAi_Kit/Monster_NBC.Update Haunter Patrol Path By Floor` (`self.Haunter`) (`self.Patrol Looping?`) (`self.Patrol Delay`))))))))))))

(fn `UserConstructionScript`)