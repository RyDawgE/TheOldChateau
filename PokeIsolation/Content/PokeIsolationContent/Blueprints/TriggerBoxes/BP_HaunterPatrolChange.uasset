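; BP_HaunterPatrolChange is a trigger box that lures the Haunter monster to the player and changes its patrol.
; Player overlap fires a DoOnce that buffs Haunter's speed and runs AIMoveTo toward the player's location.
; When the move ends, it assigns a preset spline path or updates patrol by player floor, then self-destructs or re-arms after cooldown.
; Escape-the-mansion mode re-arms the box and applies escape speed buffs only.
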(event `self.ReceiveBeginPlay`
  ;[0.06771 0.06771 0.06771] Get and Save Haunter in Map WIll need to be ran again if Haunter is destroyed for some reason
  (bind _outactors (`GameplayStatics.GetAllActorsWithTag` "Haunter"))
  (bind _asmonster_nbc (cast `/Game/MonsterAi_Kit/Monster_NBC` (`|GetArrayItem` _outactors)))
  (set `self.Haunter` _asmonster_nbc)
  (bind _asbp_pk_o_character (cast `/Game/PokeIsolationContent/Framework/Player/BP_PkO_Character` (`GameplayStatics.GetPlayerCharacter` 0)))
  (set `self.As BP Pk O Character` _asbp_pk_o_character))

(event `Reset Trigger Box`
  (goto _label :!via `Reset`))

(event `self.Box.OnComponentBeginOverlap`
  (params (OverlappedComponent :type "PrimitiveComponent Object Reference") (OtherActor :type "Actor Object Reference") (OtherComp :type "PrimitiveComponent Object Reference") (OtherBodyIndex :type Integer) (bFromSweep :type Boolean) (SweepResult :type "HitResult Structure (by ref)"))
  (if (`self.Active`)
    (bind _asbp_pk_o_character (cast `/Game/PokeIsolationContent/Framework/Player/BP_PkO_Character` OtherActor))
    (`/Engine/EditorBlueprintResources/StandardMacros.DoOnce` false :!label _label
      (:`Completed`
        (`KismetSystemLibrary.PrintString` "Haunter is on its way!!!" true true (struct :`R` 1.0 :`B` 0.355946 :`A` 1.0) 20.0)
        (if (not (`self.EscapeTheMansionActive`))
          (`/Game/MonsterAi_Kit/Monster_NBC.Jump Scare Buffs` (`self.Haunter`) (`self.Patrol State Speed`) (`self.Chase Speed`) (`self.Duration`) 0.0)
          (`AITask_MoveTo.AIMoveTo` (`AIBlueprintHelperLibrary.GetAIController` (`self.Haunter`)) (`/Game/PokeIsolationContent/Framework/Player/BP_PkO_Character.GetPlayerLocation` _asbp_pk_o_character) null -1.0 "Default" "Default" true false
            (:`OnRequestFailed`
              (`/Engine/EditorBlueprintResources/StandardMacros.IsValid` (`self.New Patrol Path`)
                (:`Is Valid`
                  (bind _output_get (set `/Game/MonsterAi_Kit/Monster_NBC.PatrolSplinePath` (`self.New Patrol Path`) (`self.Haunter`) :!label _label_2))
                  (`KismetSystemLibrary.PrintString` (`KismetSystemLibrary.GetDisplayName` _output_get)))
                (:`Is Not Valid`
                  (`/Game/MonsterAi_Kit/Monster_NBC.Update Haunter Patrol Path By Player Location` (`self.Haunter`) (`/Game/PokeIsolationContent/Framework/Player/BP_PkO_Character.PlayerLocation` (`self.As BP Pk O Character`)) (`self.Patrol Looping?`) (`self.Patrol Delay`))
                  (if (`self.DestroyAfterTriggered`)
                    (`self.K2_DestroyActor`)
                    (`KismetSystemLibrary.PrintString` "Haunter Patrol Change Box Was Destroyed" true true (struct :`R` 1.0 :`G` 0.271004 :`A` 1.0) 10.0 :!label _label_3)
                    (else
                      (`KismetSystemLibrary.Delay` (`self.Cooldown`))
                      (`self.Reset Trigger Box`))))))
            (:`OnMoveFinished`
              (`/Engine/EditorBlueprintResources/StandardMacros.IsValid` (`self.New Patrol Path`)
                (:`Is Valid`
                  (goto _label_2))
                (:`Is Not Valid`
                  (`/Game/MonsterAi_Kit/Monster_NBC.Update Haunter Patrol Path By Player Location` (`self.Haunter`) (`/Game/PokeIsolationContent/Framework/Player/BP_PkO_Character.PlayerLocation` (`self.As BP Pk O Character`)) (`self.Patrol Looping?`) (`self.Patrol Delay`))
                  (if (`self.DestroyAfterTriggered`)
                    (`self.K2_DestroyActor`)
                    (goto _label_3)
                    (else
                      (`KismetSystemLibrary.Delay` (`self.Cooldown`))
                      (`self.Reset Trigger Box`)))))))
          (else
            (`/Game/MonsterAi_Kit/Monster_NBC.Jump Scare Buffs` (`self.Haunter`) (`self.Escape Initial Speed`) (`self.Escape Chase Speed`) (`self.Escape Duration`) 0.0)))))))

(event `Escape The Mansion Enabled`
  ;[1 1 1] escape the mansion resets all boxes
  (`self.Reset Trigger Box`)
  (set `self.Active` true)
  (set `self.EscapeTheMansionActive` true))

(fn `UserConstructionScript`)