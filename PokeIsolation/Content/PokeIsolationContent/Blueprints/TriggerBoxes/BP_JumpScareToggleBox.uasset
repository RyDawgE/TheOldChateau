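; Trigger box that switches on Haunter jump scares once the player's EscapeTheMansion event fires.
; BeginPlay caches tagged East, West and Final jump scare actors; the escape event activates the Final group and arms the box.
; When the player leaves the box, the normalized world X direction from its center selects whether East or West scares activate.
; Either choice turns off the box's overlaps until ResetJumpScareController restores them.
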(event `self.ReceiveBeginPlay`
  (bind _outactors (`GameplayStatics.GetAllActorsOfClassWithTag` "/Game/PokeIsolationContent/Blueprints/TriggerBoxes/BP_HaunterJumpScare.BP_HaunterJumpScare_C" "EastJumpScare"))
  (set `self.EastJumpScare` _outactors)
  (bind _outactors_2 (`GameplayStatics.GetAllActorsOfClassWithTag` "/Game/PokeIsolationContent/Blueprints/TriggerBoxes/BP_HaunterJumpScare.BP_HaunterJumpScare_C" "WestJumpScare"))
  (set `self.WestJumpScare` _outactors_2)
  (bind _outactors_3 (`GameplayStatics.GetAllActorsOfClassWithTag` "/Game/PokeIsolationContent/Blueprints/TriggerBoxes/BP_HaunterJumpScare.BP_HaunterJumpScare_C" "FinalJumpScare"))
  (set `self.FinalHaunt` _outactors_3)
  (bind _asbp_pk_o_character (cast `/Game/PokeIsolationContent/Framework/Player/BP_PkO_Character` (`GameplayStatics.GetPlayerCharacter` 0)))
  (add `/Game/PokeIsolationContent/Framework/Player/BP_PkO_Character.EscapeTheMansion` _asbp_pk_o_character (delegate `ActivateJumpScareTriggerController`)))

(event `ActivateJumpScareTriggerController`
  (for _array_element (`self.FinalHaunt`)
    (`/Game/PokeIsolationContent/Blueprints/TriggerBoxes/BP_HaunterJumpScare.Activate` _array_element)
    (set `PrimitiveComponent.bGenerateOverlapEvents` true (`self.Box`))
    (set `self.Active` true)
    (`KismetSystemLibrary.PrintString` "JUMP SCARE CONTROLLER IS ACVTIVE" true true (struct :`R` 1.0 :`G` 0.208337 :`A` 1.0) 10.0)))

(event `self.Box.OnComponentEndOverlap`
  (params (OverlappedComponent :type "PrimitiveComponent Object Reference") (OtherActor :type "Actor Object Reference") (OtherComp :type "PrimitiveComponent Object Reference") (OtherBodyIndex :type Integer))
  (if (`self.Active`)
    (bind _asbp_pk_o_character (cast `/Game/PokeIsolationContent/Framework/Player/BP_PkO_Character` OtherActor))
    (bind _returnvalue_x (`KismetMathLibrary.BreakVector` (`KismetMathLibrary.Normal` (- (`self.K2_GetActorLocation` _asbp_pk_o_character) (`self.K2_GetActorLocation`)))))
    (if (< _returnvalue_x -0.8)
      (for _array_element (`self.EastJumpScare`)
        (`/Game/PokeIsolationContent/Blueprints/TriggerBoxes/BP_HaunterJumpScare.Activate` _array_element)
        (set `PrimitiveComponent.bGenerateOverlapEvents` false (`self.Box`)))
      (`KismetSystemLibrary.PrintString` "East Jump Scare is Active" true true (struct :`G` 0.270756 :`B` 1.0 :`A` 1.0) 10.0)
      (elif (> _returnvalue_x 0.4)
        (for _array_element_2 (`self.WestJumpScare`)
          (`/Game/PokeIsolationContent/Blueprints/TriggerBoxes/BP_HaunterJumpScare.Activate` _array_element_2)
          (set `PrimitiveComponent.bGenerateOverlapEvents` false (`self.Box`)))
        (`KismetSystemLibrary.PrintString` "West Jump Scare is Active" true true (struct :`G` 0.269486 :`B` 1.0 :`A` 1.0) 10.0)))))

(event `reset overlap`)

(event `ResetJumpScareController`
  (set `PrimitiveComponent.bGenerateOverlapEvents` true (`self.Box`)))

(fn `UserConstructionScript`)