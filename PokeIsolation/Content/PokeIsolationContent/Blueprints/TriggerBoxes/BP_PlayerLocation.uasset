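; BP_PlayerLocation is a trigger volume that tracks which level area the player and the Haunter monster are in.
; Each box holds a location enum value and, on overlap, writes it to the player character's PlayerLocation or the monster's HaunterLocation.
; It updates only when the stored value differs, then prints a debug message naming the new location.
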(event `self.Box.OnComponentBeginOverlap`
  (params (OverlappedComponent :type "PrimitiveComponent Object Reference") (OtherActor :type "Actor Object Reference") (OtherComp :type "PrimitiveComponent Object Reference") (OtherBodyIndex :type Integer) (bFromSweep :type Boolean) (SweepResult :type "HitResult Structure (by ref)"))
  (bind _asbp_pk_o_character (cast `/Game/PokeIsolationContent/Framework/Player/BP_PkO_Character` OtherActor)
    (:`then`
      (if (`|EnumInequality` (`/Game/PokeIsolationContent/Framework/Player/BP_PkO_Character.PlayerLocation` _asbp_pk_o_character) (`self.LocationOfThisBox`))
        (set `/Game/PokeIsolationContent/Framework/Player/BP_PkO_Character.PlayerLocation` (`self.LocationOfThisBox`) _asbp_pk_o_character)
        (`KismetSystemLibrary.PrintString` (`KismetTextLibrary.Conv_TextToString` (`|FormatText` "Player is now on the {currentLevel}" (`|GetEnumeratorNameAsString` (`self.LocationOfThisBox`)))))))
    (:`CastFailed`
      (bind _asmonster_nbc (cast `/Game/MonsterAi_Kit/Monster_NBC` OtherActor))
      (if (`|EnumInequality` (`/Game/MonsterAi_Kit/Monster_NBC.HaunterLocation` _asmonster_nbc) (`self.LocationOfThisBox`))
        (set `/Game/MonsterAi_Kit/Monster_NBC.HaunterLocation` (`self.LocationOfThisBox`) _asmonster_nbc)
        (`KismetSystemLibrary.PrintString` (`KismetTextLibrary.Conv_TextToString` (`|FormatText` "Haunter is now on the {currentLevel}" (`|GetEnumeratorNameAsString` (`self.LocationOfThisBox`)))))))))

(fn `UserConstructionScript`)