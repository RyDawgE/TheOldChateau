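; BP_PKO_HUD is the HUD that owns the main on-screen widget and the item inspect panel.
; BeginPlay creates the main widget and binds to the player character's flashlight event.
; First flashlight use plays the widget's fade animation if the GameInstance tooltip flag is set, then clears that flag.
; ShowHideInspectWidget toggles the inspect panel, creating it with name, description and collectable data or removing it.
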(event `self.ReceiveBeginPlay`
  (bind _returnvalue (`|CreateWidget` "/Game/PokeIsolationContent/Widgets/W_MainWidget.W_MainWidget_C" (`GameplayStatics.GetPlayerController` 0)))
  (bind _output_get (set `self.MainWidgetReference` _returnvalue))
  (`UserWidget.AddToViewport` _output_get 0)
  (bind _asbp_pk_o_character (cast `/Game/PokeIsolationContent/Framework/Player/BP_PkO_Character` (`GameplayStatics.GetPlayerCharacter` 0)))
  (add `/Game/PokeIsolationContent/Framework/Player/BP_PkO_Character.UseFlashlightEvent` _asbp_pk_o_character (delegate `UseFlashlight`)))

(event `UseFlashlight`
  (bind _asbp_pko_game_instance (cast `/Game/PokeIsolationContent/Framework/Game/BP_PKO_GameInstance` (`GameplayStatics.GetGameInstance`)))
  (`/Engine/EditorBlueprintResources/StandardMacros.DoOnce` (not (`/Game/PokeIsolationContent/Framework/Game/BP_PKO_GameInstance.ShowFlashlightToolTip` _asbp_pko_game_instance))
    (:`Completed`
      (`/Game/PokeIsolationContent/Widgets/W_MainWidget.PlayFadeAnimation` (`self.MainWidgetReference`))
      (set `/Game/PokeIsolationContent/Framework/Game/BP_PKO_GameInstance.ShowFlashlightToolTip` false _asbp_pko_game_instance))))

(event `ShowHideInspectWidget`
  (params (Name :type Text) (Description :type Text) (Collectable :type Boolean))
  (bind _inspectinfowidgetref (`self.InspectInfoWidgetRef`))
  ;[1 1 1] Show / Hide Inspect Widget
  (`/Engine/EditorBlueprintResources/StandardMacros.IsValid` _inspectinfowidgetref
    (:`Is Valid`
      (`Widget.RemoveFromParent` _inspectinfowidgetref)
      (set `self.InspectInfoWidgetRef` null))
    (:`Is Not Valid`
      (bind _returnvalue (`|CreateWidget` "/Game/PokeIsolationContent/Widgets/W_InspectInfo.W_InspectInfo_C" (`GameplayStatics.GetPlayerController` 0) Name Description Collectable))
      (bind _output_get (set `self.InspectInfoWidgetRef` _returnvalue))
      (`UserWidget.AddToViewport` _output_get 0)
      (`WidgetBlueprintLibrary.SetFocusToGameViewport`))))

(fn `UserConstructionScript`)