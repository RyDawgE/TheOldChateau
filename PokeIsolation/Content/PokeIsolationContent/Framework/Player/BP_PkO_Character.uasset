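; First-person player character for a horror mansion game with Gastly monsters, handling movement, inspection, collection, hiding and pausing.
; Interaction line-traces, spawns a temporary sphere and picks the nearest valid actor to inspect, use or hide in.
; Collected keys and puzzle pieces notify the HUD, with three pieces triggering the escape objective.
; Sprinting reports noise to AI, while the flickerable flashlight periodically traces to damage Gastlys.
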(event `EnhancedInput|/Game/FirstPerson/Input/Actions/IA_Look`
  (params (ActionValue :type "Vector2D Structure") (ElapsedSeconds :type "Float (double-precision)") (TriggeredSeconds :type "Float (double-precision)") (InputAction :type "InputAction Object Reference" :default "/Game/FirstPerson/Input/Actions/IA_Look.IA_Look"))
  (bind _inspectingactor (`self.InspectingActor`))
  (bind _mesh (`/Game/PokeIsolationContent/Blueprints/Interaction/Items/BP_InspectItemBase.Mesh` _inspectingactor))
  (:`Triggered`
    (`|ExecutionSequence`
      (:`then_0`
        (if (`self.CanLook`)
          (`self.AddControllerYawInput` ActionValue_X)
          (`self.AddControllerPitchInput` ActionValue_Y)))
      (:`then_1`
        (`/Engine/EditorBlueprintResources/StandardMacros.IsValid` _inspectingactor
          (:`Is Valid`
            (`SceneComponent.K2_AddLocalRotation` _mesh (`KismetMathLibrary.MakeRotator` 0.0 0.0 ActionValue_X) false false)
            (`SceneComponent.K2_AddWorldRotation` _mesh (`KismetMathLibrary.MakeRotator` 0.0 ActionValue_Y) false false)))))))

(event `self.ReceiveBeginPlay`
  (`parent.ReceiveBeginPlay`)
  (bind _returnvalue (`|CreateWidget` "/Game/PokeIsolationContent/Widgets/W_FadeFromBlack.W_FadeFromBlack_C"))
  (`UserWidget.AddToViewport` _returnvalue 0)
  (bind _asbp_pko_hud (cast `/Game/PokeIsolationContent/Framework/HUD/BP_PKO_HUD` (`PlayerController.GetHUD` (`GameplayStatics.GetPlayerController` 0))))
  (set `self.Main Widget Reference` (`/Game/PokeIsolationContent/Framework/HUD/BP_PKO_HUD.MainWidgetReference` _asbp_pko_hud)))

(event `SpawnGhastly`
  (if (< (`self.CurrentGhastlys`) (`self.MaxGhastlys`))
    (`|SpawnActorFromClass` "/Game/Hide_easily/Blueprints/AI/BP_AI-Gastly.BP_AI-Gastly_C" (`KismetMathLibrary.MakeTransform` (`NavigationSystemV1.K2_GetRandomReachablePointInRadius` (`self.K2_GetActorLocation`) 2400.0 null null)) "AlwaysSpawn" "MultiplyWithRoot" null true 200.0 200.0 400.0 1.0 1200.0 false null)
    (`/Engine/EditorBlueprintResources/StandardMacros.IncrementInt` (`self.CurrentGhastlys`))))

(event `/Game/Hide_easily/Blueprints/HideUnderBed/BI_HideUnderBed.StopFootsteps`
  ;[1 1 1 1 25] Movement
  (`TimelineComponent.Stop` (`self.Footsteps_TL`))
  (set `self.isSprinting` false))

(event `OnFlickerFlashLight`
  (params (FlickerFlashLight :type Boolean))
  ;[1 1 1] Flicker Flash Light
  (if (`self.bFlashlightEnabled`)
    (bind _output_get (set `self.FlashLightFlicker` FlickerFlashLight))
    (if _output_get
      (`/Engine/EditorBlueprintResources/StandardMacros.FlipFlop`
        (:`A`
          (`LightComponent.SetIntensity` (`self.SpotLight_V2`) (`KismetMathLibrary.RandomFloatInRange` 1000.0 200000.0))
          (`KismetSystemLibrary.Delay` (`KismetMathLibrary.RandomFloatInRange` 0.1 0.2))
          (if (== (`self.NumberOfFlickers`) 2)
            (`KismetSystemLibrary.Delay` 4.0)
            (`self.OnFlickerFlashLight` true)
            (else
              (`self.OnFlickerFlashLight` true))))
        (:`B`
          (`LightComponent.SetIntensity` (`self.SpotLight_V2`) 0.0)
          (`KismetSystemLibrary.Delay` (`KismetMathLibrary.RandomFloatInRange` 0.1 0.2))
          (`self.OnFlickerFlashLight` true)
          (`/Engine/EditorBlueprintResources/StandardMacros.IncrementInt` (`self.NumberOfFlickers`))))
      (else
        (`LightComponent.SetIntensity` (`self.SpotLight_V2`) 0.0)
        (`KismetSystemLibrary.Delay` (`KismetMathLibrary.RandomFloatInRange` 0.1 0.2))
        (`LightComponent.SetIntensity` (`self.SpotLight_V2`) (`KismetMathLibrary.RandomFloatInRange` 20000.0 100000.0))))))

(event `EnhancedInput|/Game/FirstPerson/Input/Actions/IA_Move`
  (params (ActionValue :type "Vector2D Structure") (ElapsedSeconds :type "Float (double-precision)") (TriggeredSeconds :type "Float (double-precision)") (InputAction :type "InputAction Object Reference" :default "/Game/FirstPerson/Input/Actions/IA_Move.IA_Move"))
  (bind _returnvalue (`self.K2_GetActorLocation`))
  (bind _footsteps_tl (`self.Footsteps_TL`))
  ;[1 1 1 1 25] Movement
  (:`Triggered`
    (`|ExecutionSequence`
      (:`then_0`
        (`/Engine/EditorBlueprintResources/StandardMacros.DoOnce` false :!label _label))
      (:`then_1`
        (`KismetSystemLibrary.Delay` 0.6)
        (goto _label :!via `Reset`))
      (:`then_2`
        (`PlayerController.ClientStartCameraShake` :`self` (`GameplayStatics.GetPlayerController` 0) :`Shake` "/Game/SICKA_mansion/Blueprints/CharacterSystem/BP_HeadbobCameraShake.BP_HeadbobCameraShake_C" :`Scale` 0.3)
        (`TimelineComponent.Play` _footsteps_tl))
      (:`then_3`
        (`/Engine/EditorBlueprintResources/StandardMacros.DoOnce` false :!label _label_2
          (:`Completed`
            (`KismetSystemLibrary.K2_SetTimerDelegate` (delegate `ResetAINotify`) 0.25)
            (if (and (not (`self.Hiding`)) (not (`self.Slowed`)) (`self.isSprinting`))
              (`GameplayStatics.PlaySoundAtLocation` "/Game/assets/Sounds/Footsteps/Footsteps_Cue.Footsteps_Cue" _returnvalue (struct) 1.0 1.0 0.0 null null self null)
              (`AISense_Hearing.ReportNoiseEvent` _returnvalue 1.0 null 1000.0)
              (`KismetSystemLibrary.PrintString` "Making Noise!" true true (struct :`R` 0.05577 :`G` 1.0 :`A` 1.0))))))))
  (:`Completed`
    (`PlayerController.ClientStopCameraShake` (`GameplayStatics.GetPlayerController` 0) "/Game/SICKA_mansion/Blueprints/CharacterSystem/BP_HeadbobCameraShake.BP_HeadbobCameraShake_C" false)
    (`TimelineComponent.Stop` _footsteps_tl)))

(event `EnhancedInput|/Game/PokeIsolationContent/Framework/Player/InputActions/IA_ToggleFlashlight`
  (params (ActionValue :type Boolean) (ElapsedSeconds :type "Float (double-precision)") (TriggeredSeconds :type "Float (double-precision)") (InputAction :type "InputAction Object Reference" :default "/Game/PokeIsolationContent/Framework/Player/InputActions/IA_ToggleFlashlight.IA_ToggleFlashlight"))
  (bind _spotlight_v2 (`self.SpotLight_V2`))
  (bind _lightbeam (`self.LightBeam`))
  ;[1 1 1] Flashlight
  (:`Started`
    (`self.UseFlashlightEvent`)
    (if (`self.bFlashlightEnabled`)
      (`GameplayStatics.PlaySoundAtLocation` "/Game/Sounds/Flashlight/SC_FlashlightToggle.SC_FlashlightToggle" (`self.GetPlayerLocation`) (struct) 0.2 1.0 0.0 null null null null)
      (`SceneComponent.SetHiddenInGame` _spotlight_v2 true false)
      (`SceneComponent.SetHiddenInGame` _lightbeam true false)
      (set `self.bFlashlightEnabled` false)
      (else
        (`GameplayStatics.PlaySoundAtLocation` "/Game/Sounds/Flashlight/SC_FlashlightToggle.SC_FlashlightToggle" (`self.GetPlayerLocation`) (struct) 0.2 1.0 0.0 null null null null)
        (`SceneComponent.SetHiddenInGame` _spotlight_v2 false false)
        (`SceneComponent.SetHiddenInGame` _lightbeam false false)
        (set `self.bFlashlightEnabled` true)))))

(event `ResetAINotify`
  ;[1 1 1 1 25] Movement
  (goto _label_2 :!via `Reset`))

(event `Update HUD`
  (params (`Used Item` :type Text))
  (`/Game/PokeIsolationContent/Widgets/W_MainWidget.Show Use Item Notify` (`self.Main Widget Reference`) `Used Item`))

(event `EnhancedInput|/Game/PokeIsolationContent/Framework/Player/InputActions/IA_Interact`
  (params (ActionValue :type Boolean) (ElapsedSeconds :type "Float (double-precision)") (TriggeredSeconds :type "Float (double-precision)") (InputAction :type "InputAction Object Reference" :default "/Game/PokeIsolationContent/Framework/Player/InputActions/IA_Interact.IA_Interact"))
  (bind (_velocity_x _velocity_y _velocity_z) (`KismetMathLibrary.BreakVector` (`MovementComponent.Velocity` (`self.CharacterMovement`))))
  (:`Started`
    (`/Engine/EditorBlueprintResources/StandardMacros.IsValid` (`self.InspectingActor`)
      (:`Is Valid`
        (`CharacterMovementComponent.SetMovementMode` (`self.CharacterMovement`) "MOVE_Walking" 0)
        (set `self.CanLook` true)
        (`/Game/PokeIsolationContent/Blueprints/Interaction/Items/BP_InspectItemBase.Inspect_PutAway` (`self.InspectingActor`))
        (set `self.InspectingActor` null))
      (:`Is Not Valid`
        (`GameplayStatics.PlaySoundAtLocation` "/Engine/VREditor/Sounds/UI/Object_PickUp.Object_PickUp" (`self.GetPlayerLocation`) (struct) 0.2 1.0 0.0 null null null null)
        (bind _was_inspectable (`self.InteractionTrace`))
        (if (and (== _velocity_z 0.0) _was_inspectable)
          (`CharacterMovementComponent.DisableMovement` (`self.CharacterMovement`))
          (set `self.CanLook` false))))))

(event `EnhancedInput|/Game/PokeIsolationContent/Framework/Player/InputActions/IA_CollectItem`
  (params (ActionValue :type Boolean) (ElapsedSeconds :type "Float (double-precision)") (TriggeredSeconds :type "Float (double-precision)") (InputAction :type "InputAction Object Reference" :default "/Game/PokeIsolationContent/Framework/Player/InputActions/IA_CollectItem.IA_CollectItem"))
  (bind _inspectingactor (`self.InspectingActor`))
  (bind _inspectingactor_2 (`self.InspectingActor`))
  ;[1 1 1] Collect Item
  (:`Started`
    (`/Engine/EditorBlueprintResources/StandardMacros.IsValid` _inspectingactor
      (:`Is Valid`
        (if (`/Game/PokeIsolationContent/Blueprints/Interaction/Items/BP_InspectItemBase.bCollectable` _inspectingactor)
          (bind _asbp_pko_hud (cast `/Game/PokeIsolationContent/Framework/HUD/BP_PKO_HUD` (`PlayerController.GetHUD` (`GameplayStatics.GetPlayerController` 0))))
          (bind _mainwidgetreference (`/Game/PokeIsolationContent/Framework/HUD/BP_PKO_HUD.MainWidgetReference` _asbp_pko_hud))
          (`/Game/PokeIsolationContent/Widgets/W_MainWidget.ShowCollectionNotify` _mainwidgetreference (`/Game/PokeIsolationContent/Blueprints/Interaction/Items/BP_InspectItemBase.Name` _inspectingactor))
          (`KismetSystemLibrary.PrintString` "Item is collected")
          ;;[0.01219 0.1823 0] If Key Add to Collected Keys and Map
          (bind _asbp_key (cast `/Game/PokeIsolationContent/Blueprints/Interaction/Items/BP_Key` _inspectingactor_2)
            (:`then`
              (`BlueprintMapLibrary.Map_Add` (`self.CollectedKeys`) (`/Game/PokeIsolationContent/Blueprints/Interaction/Items/BP_Key.KeyID` _asbp_key) _asbp_key)
              (bind _result (`/Engine/EditorBlueprintResources/StandardMacros.IncrementInt` (`self.CollectedKeyCount`))
                (:`  `
                  (`self.UpdateKeyCount` (`/Game/PokeIsolationContent/Blueprints/Interaction/Items/BP_InspectItemBase.Name` _asbp_key) _result))))
            (:`CastFailed`
              ;;[0.01219 0.1823 0] If Puzzle Add to Collected Puzzle and if 3 Update Objective
              (bind _asbp_puzzle_item (cast `/Game/PokeIsolationContent/Blueprints/Interaction/Items/BP_PuzzleItem` _inspectingactor_2)
                (:`then`
                  (bind _result_2 (`/Engine/EditorBlueprintResources/StandardMacros.IncrementInt` (`self.CollectedPuzzleCount`))
                    (:`  `
                      (bind _name (`/Game/PokeIsolationContent/Blueprints/Interaction/Items/BP_InspectItemBase.Name` _asbp_puzzle_item))
                      (`/Game/PokeIsolationContent/Widgets/W_MainWidget.ShowCollectionNotify` _mainwidgetreference _name)
                      (`self.UpdatePuzzlePieceCount` _name _result_2)
                      (if (== (`self.CollectedPuzzleCount`) 3)
                        (`/Game/PokeIsolationContent/Widgets/W_MainWidget.ShowObjectiveNotify` (`/Game/PokeIsolationContent/Framework/HUD/BP_PKO_HUD.MainWidgetReference` _asbp_pko_hud) "Escape the mansion")
                        (`GameplayStatics.PlaySound2D` "/Game/Sounds/Haunter/ES_Monster_GroanWReverb.ES_Monster_GroanWReverb" 1.3 0.8 0.0 null null)
                        (`self.EscapeTheMansion`)))))
                (:`CastFailed`
                  _))))
          (`GameplayStatics.PlaySoundAtLocation` "/Game/Sounds/Items/SC_TakeItem.SC_TakeItem" (`self.GetPlayerLocation`) (struct) 1.0 1.0 0.0 null null null null)
          (`self.K2_DestroyActor` (`self.InspectingActor`))
          (`/Game/PokeIsolationContent/Framework/HUD/BP_PKO_HUD.ShowHideInspectWidget` _asbp_pko_hud "" "" false)
          (`CharacterMovementComponent.SetMovementMode` (`self.CharacterMovement`) "MOVE_Walking" 0)
          (set `self.CanLook` true)
          (set `self.InspectingActor` null))))))

(event `EnhancedInput|/Game/PokeIsolationContent/Framework/Player/InputActions/IA_ZoomItem`
  (params (ActionValue :type "Float (double-precision)") (ElapsedSeconds :type "Float (double-precision)") (TriggeredSeconds :type "Float (double-precision)") (InputAction :type "InputAction Object Reference" :default "/Game/PokeIsolationContent/Framework/Player/InputActions/IA_ZoomItem.IA_ZoomItem"))
  (bind _returnvalue (* (* ActionValue 10.0) -1.0))
  (bind _relativelocation_x (`KismetMathLibrary.BreakVector` (`SceneComponent.RelativeLocation` (`self.InspectPoint`))))
  (:`Started`
    (`/Engine/EditorBlueprintResources/StandardMacros.IsValid` (`self.InspectingActor`)
      (:`Is Valid`
        (if (`KismetMathLibrary.InRange_FloatFloat` (+ _relativelocation_x _returnvalue) 30.0 150.0)
          (`SceneComponent.K2_SetRelativeLocation` (`self.InspectPoint`) (+ (`SceneComponent.RelativeLocation` (`self.InspectPoint`)) (`KismetMathLibrary.MakeVector` _returnvalue)) false false)
          (bind (_direction _lerpvalue) (`Timeline|TL_SetInspectZoom` :!via `PlayFromStart`)
            (:`Update`
              (`/Engine/EditorBlueprintResources/StandardMacros.IsValid` (`self.InspectingActor`)
                (:`Is Valid`
                  (`SceneComponent.K2_SetWorldLocation` (`/Game/PokeIsolationContent/Blueprints/Interaction/Items/BP_InspectItemBase.Mesh` (`self.InspectingActor`)) (`KismetMathLibrary.VLerp` (`SceneComponent.K2_GetComponentLocation` (`/Game/PokeIsolationContent/Blueprints/Interaction/Items/BP_InspectItemBase.Mesh` (`self.InspectingActor`))) (`SceneComponent.K2_GetComponentLocation` (`self.InspectPoint`)) _lerpvalue) false false))))))))))

(event `/Game/Hide_easily/Blueprints/HideUnderBed/BI_HideUnderBed.ChangeControl`
  (params (UsePawnControlRotation :type Boolean))
  ;[0.01042 0.006851 0.002351] Interface For Hide Under Bed
  (`/Game/Hide_easily/Blueprints/HideUnderBed/AC_HideUnderBed.ChangeControlRotation` (`self.AC_HideUnderBed`) UsePawnControlRotation (`self.FirstPersonCamera`)))

(event `EnhancedInput|/Game/PokeIsolationContent/Framework/Player/InputActions/IA_Sprint`
  (params (ActionValue :type Boolean) (ElapsedSeconds :type "Float (double-precision)") (TriggeredSeconds :type "Float (double-precision)") (InputAction :type "InputAction Object Reference" :default "/Game/PokeIsolationContent/Framework/Player/InputActions/IA_Sprint.IA_Sprint"))
  (bind _footsteps_tl (`self.Footsteps_TL`))
  ;[1 1 1 1 25] Sprint
  (:`Started`
    (if (not (`self.Slowed`))
      (bind _output_get (set `self.isSprinting` true))
      (`self.UpdateMovementSpeed`)
      (if _output_get
        (`TimelineComponent.SetPlayRate` _footsteps_tl 2.5))))
  (:`Canceled`
    (set `self.isSprinting` false :!label _label_3)
    (`self.UpdateMovementSpeed`)
    (`TimelineComponent.SetPlayRate` _footsteps_tl 1.0))
  (:`Completed`
    (goto _label_3)))

(event `/Game/Hide_easily/Blueprints/HideUnderBed/BI_HideUnderBed.SetAnimationMode`
  ;[0.01042 0.006851 0.002351] Interface For Hide Under Bed
  (`/Game/Hide_easily/Blueprints/HideUnderBed/AC_HideUnderBed.ServerSetAnimationMode` (`self.AC_HideUnderBed`) (`self.Mesh`)))

(event `EnhancedInput|/Game/PokeIsolationContent/Framework/Player/InputActions/IA_PauseGame`
  (params (ActionValue :type Boolean) (ElapsedSeconds :type "Float (double-precision)") (TriggeredSeconds :type "Float (double-precision)") (InputAction :type "InputAction Object Reference" :default "/Game/PokeIsolationContent/Framework/Player/InputActions/IA_PauseGame.IA_PauseGame"))
  (bind _returnvalue (`GameplayStatics.GetPlayerController` 0))
  ;[1 1 1] Pause Game
  (:`Started`
    (if (not (`self.bPauseMenuOpen`))
      (set `self.bPauseMenuOpen` true)
      (bind _returnvalue_2 (`|CreateWidget` "/Game/PokeIsolationContent/Widgets/W_PauseMenu.W_PauseMenu_C" _returnvalue))
      (bind _output_get (set `self.PauseMenuWdiget` _returnvalue_2))
      (`UserWidget.AddToViewport` _output_get 0)
      (`WidgetBlueprintLibrary.SetInputMode_GameAndUIEx` _returnvalue (`self.PauseMenuWdiget`))
      (set `PlayerController.bShowMouseCursor` true (`GameplayStatics.GetPlayerController` 0))
      (`GameplayStatics.SetGamePaused` true)
      (else
        (set `self.bPauseMenuOpen` false)
        (`Widget.RemoveFromParent` (`self.PauseMenuWdiget`))
        (`GameplayStatics.SetGamePaused` false)
        (`WidgetBlueprintLibrary.SetInputMode_GameOnly` _returnvalue)
        (set `PlayerController.bShowMouseCursor` false (`GameplayStatics.GetPlayerController` 0))))))

(event `/Game/Hide_easily/Blueprints/HideUnderBed/BI_HideUnderBed.RunHide`
  ;[0.01042 0.006851 0.002351] Interface For Hide Under Bed
  (`TimelineComponent.Stop` (`self.Footsteps_TL`))
  (`/Game/Hide_easily/Blueprints/HideUnderBed/AC_HideUnderBed.ServerRunHideAnimation` (`self.AC_HideUnderBed`) (`self.FirstPersonCamera`) (`self.Mesh`) (`self.CharacterMovement`) (`GameplayStatics.GetPlayerController` 0)))

(event `Slow Debuff`
  (params (`New Walk Speed` :type "Float (single-precision)") (Duration :type "Float (single-precision)"))
  ;[1 1 1] Slow Debuff
  (if (not (`self.Slowed`))
    (set `self.Slowed` true)
    (`self.UpdateMovementSpeed`)
    (`KismetSystemLibrary.K2_SetTimerDelegate` (delegate `Restore Default Move Speed`) Duration)))

(event `/Game/Hide_easily/Blueprints/HideUnderBed/BI_HideUnderBed.RunUnhide`
  ;[0.01042 0.006851 0.002351] Interface For Hide Under Bed
  (`/Game/Hide_easily/Blueprints/HideUnderBed/AC_HideUnderBed.ServerRunUnhideAnimation` (`self.AC_HideUnderBed`) (`GameplayStatics.GetPlayerController` 0) (`self.Mesh`) (`self.FirstPersonCamera`) (`self.CharacterMovement`)))

(event `Restore Default Move Speed`
  ;[1 1 1] Restore Speed to default
  (set `self.Slowed` false)
  (`self.UpdateMovementSpeed`))

(event `/Game/Hide_easily/Blueprints/HideUnderBed/BI_HideUnderBed.UpdateHide`
  (`/Engine/EditorBlueprintResources/StandardMacros.FlipFlop`
    (:`A`
      (set `self.Hiding` true))
    (:`B`
      (set `self.Hiding` false))))

(event `self.ReceiveTick`
  (params (DeltaSeconds :type "Float (single-precision)"))
  (bind _firstpersoncamera (`self.FirstPersonCamera`))
  (bind _flashlightdamage (`self.FlashLightDamage`))
  (bind _returnvalue (`SceneComponent.K2_GetComponentLocation` _firstpersoncamera))
  ;[1 1 1] Check if Pointing at Gastly
  (`KismetSystemLibrary.Delay` 1.0)
  (if (`self.bFlashlightEnabled`)
    (bind _outhit (`KismetSystemLibrary.LineTraceSingle` _returnvalue (+ _returnvalue (* (`KismetMathLibrary.GetForwardVector` (`SceneComponent.K2_GetComponentRotation` _firstpersoncamera)) (750.0 750.0 750.0))) "TraceTypeQuery1" false (`|MakeArray` self :!type "Actor Object Reference")))
    (bind _asmonster_gastly_ai (cast `/Game/MonsterAi_Kit/Monster_GastlyAi` (`.HitActor` (`GameplayStatics.BreakHitResult` _outhit))))
    (`/Game/MonsterAi_Kit/Monster_NBC.MTK_Get_Damage` _asmonster_gastly_ai _flashlightdamage self)
    (`KismetSystemLibrary.PrintString` (`KismetTextLibrary.Conv_TextToString` (`|FormatText` "You did {damage} to Gastly" _flashlightdamage)))))

(fn `FootstepTry`
  (bind _returnvalue (`self.K2_GetActorLocation`))
  (bind _finished (`self.TraceFootSteps`))
  (if _finished
    (`GameplayStatics.PlaySoundAtLocation` "/Game/assets/Sounds/Footsteps/Footsteps_Cue.Footsteps_Cue" _returnvalue (struct) 1.5 1.0 0.0 null null self null)
    (if (`self.isSprinting`)
      (`AISense_Hearing.ReportNoiseEvent` _returnvalue 1.0 self 1500.0))))

(fn `GetPlayerLocation`
  (returns (ReturnValue :type "Vector Structure"))
  (return (`self.K2_GetActorLocation`)))

(fn `InteractionTrace`
  (returns (`Was Inspectable` :type Boolean))
  (locals (ReturnValue :type Boolean) (FilteredOverlaps :type "Array of Actor Object Reference"))
  (bind _firstpersoncamera (`self.FirstPersonCamera`))
  (bind _returnvalue (`SceneComponent.K2_GetComponentLocation` _firstpersoncamera))
  (bind (_velocity_x _velocity_y _velocity_z) (`KismetMathLibrary.BreakVector` (`MovementComponent.Velocity` (`self.CharacterMovement`))))
  (bind _outhit (`KismetSystemLibrary.LineTraceSingle` _returnvalue (+ _returnvalue (* (`KismetMathLibrary.GetForwardVector` (`SceneComponent.K2_GetComponentRotation` _firstpersoncamera)) (200.0 200.0 200.0))) "TraceTypeQuery1" false (`|MakeArray` self :!type "Actor Object Reference") "ForDuration"))
  (bind (_bblockinghit _binitialoverlap _time _distance _location _impactpoint _normal _impactnormal _physmat _hitactor _hitcomponent _hitbonename _bonename _hititem _elementindex _faceindex _tracestart _traceend) (`GameplayStatics.BreakHitResult` _outhit))
  (bind _returnvalue_2 (`KismetMathLibrary.SelectVector` _impactpoint _traceend (`KismetSystemLibrary.IsValid` _hitactor)))
  (bind _returnvalue_3 (`|SpawnActorFromClass` "/Script/Engine.TriggerSphere" (`KismetMathLibrary.MakeTransform` _returnvalue_2) "AlwaysSpawn" "MultiplyWithRoot" null null))
  (for _array_element (`self.GetOverlappingActors` _returnvalue_3 null)
    (`|ExecutionSequence`
      (:`then_0`
        (bind _asbp_interaction_door (cast `/Game/PokeIsolationContent/Blueprints/Interaction/Doors/BP_Interaction_Door` _array_element))
        (`KismetArrayLibrary.Array_Add` (`local.FilteredOverlaps`) _asbp_interaction_door))
      (:`then_1`
        (bind _asbp_inspect_item_base (cast `/Game/PokeIsolationContent/Blueprints/Interaction/Items/BP_InspectItemBase` _array_element))
        (`KismetArrayLibrary.Array_Add` (`local.FilteredOverlaps`) _asbp_inspect_item_base))
      (:`then_2`
        (if (`KismetSystemLibrary.DoesImplementInterface` _array_element "/Game/PokeIsolationContent/Blueprints/Interaction/BPI_Interaction.BPI_Interaction_C")
          (`KismetArrayLibrary.Array_Add` (`local.FilteredOverlaps`) _array_element)))))
  (`|ExecutionSequence`
    (:`then_0`
      (bind (_distance_2 _returnvalue_4) (`GameplayStatics.FindNearestActor` _returnvalue_2 (`local.FilteredOverlaps`)))
      (bind _asbp_inspect_item_base_2 (cast `/Game/PokeIsolationContent/Blueprints/Interaction/Items/BP_InspectItemBase` _returnvalue_4)
        (:`then`
          (if (and (`KismetSystemLibrary.DoesImplementInterface` _returnvalue_4 "/Game/PokeIsolationContent/Blueprints/Interaction/BPI_Interaction.BPI_Interaction_C") (== _velocity_z 0.0))
            (set `self.InspectingActor` _asbp_inspect_item_base_2)
            (message `/Game/PokeIsolationContent/Blueprints/Interaction/BPI_Interaction.OnInteract` _returnvalue_4 self)
            (set `local.ReturnValue` true)
            (else
              (set `local.ReturnValue` false))))
        (:`CastFailed`
          (message `/Game/PokeIsolationContent/Blueprints/Interaction/BPI_Interaction.OnInteract` _returnvalue_4 self)
          (bind _asbp_pk_o_player_controller (cast `/Game/PokeIsolationContent/Blueprints/GameModeandController/BP_PkO_PlayerController` (`GameplayStatics.GetPlayerController` 0)))
          (`/Game/PokeIsolationContent/Blueprints/GameModeandController/BP_PkO_PlayerController.ToggleHideEvent` _asbp_pk_o_player_controller _returnvalue_4))))
    (:`then_1`
      (`self.K2_DestroyActor` _returnvalue_3)
      (return (`local.ReturnValue`)))))

(fn `ToggleViewRestriction`
  (params (bRestrict :type Boolean) (Actor :type "Actor Object Reference"))
  (bind _returnvalue (`GameplayStatics.GetPlayerCameraManager` 0))
  (bind (_returnvalue_roll _returnvalue_pitch _returnvalue_yaw) (`KismetMathLibrary.BreakRotator` (`self.K2_GetActorRotation` Actor)))
  (bind _returnvalue_2 (`GameplayStatics.GetPlayerCameraManager` 0))
  (bind _returnvalue_3 (`GameplayStatics.GetPlayerCameraManager` 0))
  (bind _returnvalue_4 (`GameplayStatics.GetPlayerCameraManager` 0))
  (if bRestrict
    (set `PlayerCameraManager.ViewPitchMin` -15.0 _returnvalue_4)
    (set `PlayerCameraManager.ViewPitchMax` 15.0 _returnvalue_4)
    (set `PlayerCameraManager.ViewYawMin` (+ _returnvalue_yaw -15.0) _returnvalue_3)
    (set `PlayerCameraManager.ViewYawMax` (+ _returnvalue_yaw 15.0) _returnvalue_3)
    (else
      (set `PlayerCameraManager.ViewPitchMin` -90.0 _returnvalue)
      (set `PlayerCameraManager.ViewPitchMax` 90.0 _returnvalue)
      (set `PlayerCameraManager.ViewYawMin` 0.0 _returnvalue_2)
      (set `PlayerCameraManager.ViewYawMax` 359.9 _returnvalue_2))))

(fn `TraceFootSteps`
  (returns (Finished :type Boolean))
  (bind _returnvalue (`self.K2_GetActorLocation`))
  (bind _capsulecomponent (`self.CapsuleComponent`))
  (bind (_x _y _z) (`KismetMathLibrary.BreakVector3f` _returnvalue))
  (bind (_outhits _returnvalue_2) (`KismetSystemLibrary.SphereTraceMulti` _returnvalue (`KismetMathLibrary.MakeVector` _x _y (- _z (`CapsuleComponent.GetScaledCapsuleHalfHeight` _capsulecomponent))) (`CapsuleComponent.GetScaledCapsuleRadius` _capsulecomponent) "TraceTypeQuery1"))
  (return _returnvalue_2))

(fn `UpdateMovementSpeed`
  (locals (SlowedSpeedPercent :type "Float (double-precision)" :default 0.8) (SprintSpeedPercent :type "Float (double-precision)" :default 3.5))
  (set `CharacterMovementComponent.MaxWalkSpeed` (* (* (`self.defaultWalkSpeed`) (`KismetMathLibrary.SelectFloat` (`local.SprintSpeedPercent`) 1.0 (and (`self.isSprinting`) (not (`self.Slowed`))))) (`KismetMathLibrary.SelectFloat` (`local.SlowedSpeedPercent`) 1.0 (`self.Slowed`))) (`self.CharacterMovement`)))

(fn `UserConstructionScript`
  (`parent.UserConstructionScript`))